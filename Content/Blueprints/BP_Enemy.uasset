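; BP_Enemy is an enemy character drawn with a flipbook sprite, providing functions for its animation states.
; UpdateAnimation picks the death flipbook when IsDead is set, otherwise walk or idle based on CharacterMovement velocity.
; Death switches the sprite to the death flipbook without setting IsDead.
; The event graph and construction script are empty, so neither function is called within this Blueprint.
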(event EventBeginPlay)

(event Collision|EventActorBeginOverlap
  (params (OtherActor :type Actor%20Object%20Reference)))

(event EventTick
  (params (DeltaSeconds :type Float%20%28single-precision%29)))

(fn ConstructionScript)

(fn Death
  (Sprite|SetFlipbook (Variables|Default|GetSprite) (Variables|Flipbooks|GetFlipbookDeath)))

(fn UpdateAnimation
  (Sprite|SetFlipbook (Variables|Default|GetSprite) (select (Variables|Default|GetIsDead) (Variables|Flipbooks|GetFlipbookDeath) (select (> (Math|Vector|VectorLength (Variables|/Script/Engine.MovementComponent|GetVelocity (Variables|Character|GetCharacterMovement))) 0.0) (Variables|Flipbooks|GetFlipbookWalk) (Variables|Flipbooks|GetFlipbookIdle)))))