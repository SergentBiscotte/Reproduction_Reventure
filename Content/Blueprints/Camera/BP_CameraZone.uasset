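; BP_CameraZone is a box trigger volume that switches the player's orthographic camera to a new zone and updates the zone name in the UI.
; The construction script sizes the box from ScaleBox.
; When a BP_Character overlaps a different zone, it passes actor-relative corner bounds and ortho width to PlayerCamera and starts the switch.
; The zone name passes through GI_GameInfo's player-name replacement before display on the game mode's widget.
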(event OnComponentBeginOverlap(BoxDetection)
  (params (OverlappedComponent :type Primitive%20Component%20Object%20Reference) (OtherActor :type Actor%20Object%20Reference) (OtherComp :type Primitive%20Component%20Object%20Reference) (OtherBodyIndex :type Integer) (bFromSweep :type Boolean) (SweepResult :type Hit%20Result%20Structure%20%28by%20ref%29))
  (bind _asbp_character (Utilities|Casting|CastToBP_Character OtherActor))
  (CallFunction|SwitchCameraZone _asbp_character))

(event EventBeginPlay)

(event Collision|EventActorBeginOverlap
  (params (OtherActor :type Actor%20Object%20Reference)))

(event EventTick
  (params (DeltaSeconds :type Float%20%28single-precision%29)))

(fn ConstructionScript
  (Components|Box|SetBoxExtent (Variables|Default|GetBoxDetection) (Variables|Default|GetScaleBox) true))

(fn SwitchCameraZone
  (params (character :type BP%20Character%20Object%20Reference))
  (if (not (== (Variables|/Game/Blueprints/BP_Character.BP_Character_C|GetActualZone character) self))
    (Variables|/Game/Blueprints/BP_Character.BP_Character_C|SetActualZone character self)
    (Utilities|FlowControl|Sequence
      (:then_0
        ;[1 1 1] Paramétrage de la caméra lors du changement de zone
        (Variables|/Game/Blueprints/Camera/BP_CameraActor.BP_CameraActor_C|SetUpLeftPoint (Variables|/Game/Blueprints/BP_Character.BP_Character_C|GetPlayerCamera character) (+ (Variables|Default|GetUpLeftPoint) (Transformation|GetActorLocation)))
        (Variables|/Game/Blueprints/Camera/BP_CameraActor.BP_CameraActor_C|SetDownRightPoint (Variables|/Game/Blueprints/BP_Character.BP_Character_C|GetPlayerCamera character) (+ (Variables|Default|GetDownRightPoint) (Transformation|GetActorLocation)))
        (Variables|/Game/Blueprints/Camera/BP_CameraActor.BP_CameraActor_C|SetnewOrthoWidth (Variables|/Game/Blueprints/BP_Character.BP_Character_C|GetPlayerCamera character) (Variables|Default|GetcameraFov))
        (Default|StartSwitchingZone (Variables|/Game/Blueprints/BP_Character.BP_Character_C|GetPlayerCamera character)))
      (:then_1
        ;[1 1 1] Changement du nom de la zone dans l'UI
        (bind _asgi_game_info (Utilities|Casting|CastToGI_GameInfo (Game|GetGameInstance)))
        (bind _newtext (Default|ReplacePlayerName _asgi_game_info (Utilities|String|ToString(Name) (Variables|Default|GetzoneName))))
        (bind _asgm_game (Utilities|Casting|CastToGM_Game (Game|GetGameMode)))
        (Rendering|Components|TextRender|SetText (Variables|/Game/UI/W_NameZone.W_NameZone_C|GetText_NameZone (Variables|/Game/Blueprints/GameModes/GM_Game.GM_Game_C|GetwNameZoneRef _asgm_game)) (Utilities|Text|ToText(String) _newtext))))))