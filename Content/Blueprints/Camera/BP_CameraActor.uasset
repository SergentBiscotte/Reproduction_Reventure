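; Orthographic 2D camera actor that follows the player on X and Z, clamped within the current zone's corner points.
; Each tick it picks classic follow, zone switch or cinematic mode, the last drifting slowly downward.
; CalculBorder uses ortho width and aspect ratio to keep the view inside the bounds.
; StartSwitchingZone restarts a timeline that blends position and ortho width toward the new framing before classic follow resumes.
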(event Custom|SwitchZoneTimeline
  (bind _progression (Timeline|TimelineSwitch Play)
    (:Update
      (Transformation|SetActorLocation (Math|Vector|Lerp(Vector) (Variables|Default|GetOldPosition) (Variables|Default|GetNewPosition) _progression) false false)
      (Class|CameraComponent|SetOrthoWidth (Variables|Default|GetCamera) (Math|Float|Lerp (Variables|/Script/Engine.CameraComponent|GetOrthoWidth (Variables|Default|GetCamera)) (Variables|Default|GetnewOrthoWidth) (/ _progression 2.0))))))

(event Custom|RestartSwitchZoneTimeline
  (bind _progression (Timeline|TimelineSwitch PlayFromStart)
    (:Update
      (Transformation|SetActorLocation (Math|Vector|Lerp(Vector) (Variables|Default|GetOldPosition) (Variables|Default|GetNewPosition) _progression) false false)
      (Class|CameraComponent|SetOrthoWidth (Variables|Default|GetCamera) (Math|Float|Lerp (Variables|/Script/Engine.CameraComponent|GetOrthoWidth (Variables|Default|GetCamera)) (Variables|Default|GetnewOrthoWidth) (/ _progression 2.0))))))

(event EventBeginPlay)

(event Collision|EventActorBeginOverlap
  (params (OtherActor :type Actor%20Object%20Reference)))

(event EventTick
  (params (DeltaSeconds :type Float%20%28single-precision%29))
  (CallFunction|UpdatePosition))

(fn ConstructionScript)

(fn UpdatePosition
  (bind _camera (Variables|Default|GetCamera))
  ;[1 1 1] Calcul de la taille de l'écran
  (bind _output_get (LocalVariables|SetdistanceCameraX (/ (Variables|/Script/Engine.CameraComponent|GetOrthoWidth _camera) 2.0)))
  (LocalVariables|SetdistanceCameraY (/ _output_get (Variables|/Script/Engine.CameraComponent|GetAspectRatio _camera)))
  (if (not (Variables|/Game/Blueprints/BP_Character.BP_Character_C|GetisInCinematicMode (Variables|Default|Getplayer)))
    (if (Variables|Default|GetisSwitchingZone)
      (CallFunction|UpdatePositionSwitchZone (LocalVariables|GetDistanceCameraX) (LocalVariables|GetDistanceCameraY))
      (else
        (CallFunction|UpdatePositionClassic (LocalVariables|GetDistanceCameraX) (LocalVariables|GetDistanceCameraY))))
    (else
      (CallFunction|UpdatePositionCinematic (LocalVariables|GetDistanceCameraX) (LocalVariables|GetDistanceCameraY)))))

(fn UpdatePositionCinematic
  (params (DistanceCameraX :type Float%20%28double-precision%29) (DistanceCameraY :type Float%20%28double-precision%29))
  (Variables|Default|SetNewPosition (- (Transformation|GetActorLocation) (Math|Vector|MakeVector 0.0 0.0 (* (Utilities|Time|GetWorldDeltaSeconds) 2e+01))))
  (CallFunction|CalculBorder DistanceCameraX DistanceCameraY)
  (Transformation|SetActorLocation (Variables|Default|GetNewPosition) false false))

(fn UpdatePositionSwitchZone
  (params (DistanceCameraX :type Float%20%28double-precision%29) (DistanceCameraY :type Float%20%28double-precision%29))
  (Variables|Default|SetNewPosition (Transformation|GetActorLocation (Variables|Default|Getplayer)))
  (CallFunction|CalculBorder DistanceCameraX DistanceCameraY)
  (if (and (Utilities|Operators|EqualEqual (Transformation|GetActorLocation) (Variables|Default|GetNewPosition) 1.0) (== (Variables|/Script/Engine.CameraComponent|GetOrthoWidth (Variables|Default|GetCamera)) (Variables|Default|GetnewOrthoWidth)))
    (Variables|Default|SetisSwitchingZone false)
    (CallFunction|UpdatePositionClassic DistanceCameraX DistanceCameraY)
    (else
      (CallFunction|SwitchZoneTimeline))))

(fn UpdatePositionClassic
  (params (DistanceCameraX :type Float%20%28double-precision%29) (DistanceCameraY :type Float%20%28double-precision%29))
  (bind _player (Variables|Default|GetPlayer))
  (bind _returnvalue (Transformation|GetActorLocation _player))
  (Utilities|FlowControl|Sequence
    (:then_0
      (Variables|Default|SetNewPosition (Math|Vector|MakeVector (.x _returnvalue) (.y (Transformation|GetActorLocation)) (.z _returnvalue)))
      (CallFunction|CalculBorder DistanceCameraX DistanceCameraY))
    (:then_1
      (Transformation|SetActorLocation (Variables|Default|GetNewPosition) false false))))

(fn StartSwitchingZone
  (Variables|Default|SetOldPosition (Transformation|GetActorLocation))
  (Variables|Default|SetisSwitchingZone true)
  (CallFunction|RestartSwitchZoneTimeline))

(fn CalculBorder
  (params (DistanceCameraX :type Float%20%28double-precision%29) (DistanceCameraY :type Float%20%28double-precision%29))
  (bind _downrightpoint (Variables|Default|GetDownRightPoint))
  (bind _upleftpoint (Variables|Default|GetUpLeftPoint))
  (bind _upleftpoint_2 (Variables|Default|GetUpLeftPoint))
  (bind _downrightpoint_2 (Variables|Default|GetDownRightPoint))
  (Utilities|FlowControl|Sequence
    (:then_0
      (if (< (- (.x (Variables|Default|GetNewPosition)) (LocalVariables|GetdistanceCameraX)) (.x _upleftpoint))
        (Variables|Default|SetNewPosition (Math|Vector|MakeVector (+ (LocalVariables|GetdistanceCameraX) (.x _upleftpoint)) (.y (Variables|Default|GetNewPosition)) (.z (Variables|Default|GetNewPosition))))))
    (:then_1
      (if (> (+ (.z (Variables|Default|GetNewPosition)) (LocalVariables|GetdistanceCameraY)) (.z _upleftpoint_2))
        (Variables|Default|SetNewPosition (Math|Vector|MakeVector (.x (Variables|Default|GetNewPosition)) (.y (Variables|Default|GetNewPosition)) (- (.z _upleftpoint_2) (LocalVariables|GetdistanceCameraY))))))
    (:then_2
      (if (> (+ (.x (Variables|Default|GetNewPosition)) (LocalVariables|GetdistanceCameraX)) (.x _downrightpoint_2))
        (Variables|Default|SetNewPosition (Math|Vector|MakeVector (- (.x _downrightpoint_2) (LocalVariables|GetdistanceCameraX)) (.y (Variables|Default|GetNewPosition)) (.z (Variables|Default|GetNewPosition))))))
    (:then_3
      (if (< (- (.z (Variables|Default|GetNewPosition)) (LocalVariables|GetdistanceCameraY)) (.z _downrightpoint))
        (Variables|Default|SetNewPosition (Math|Vector|MakeVector (.x (Variables|Default|GetNewPosition)) (.y (Variables|Default|GetNewPosition)) (+ (.z _downrightpoint) (LocalVariables|GetdistanceCameraY))))))))