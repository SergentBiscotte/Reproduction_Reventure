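; BP_Collectible is a sprite item that the player picks up and wears, at a cost to jump height.
; Interact or sprite overlap, each behind its own DoOnce, freezes player movement and starts the collect animation.
; Two timelines lerp the item above the player, then, after a short delay, down onto them.
; EquipItem then copies the sprite onto BP_Character at an offset, lowers JumpZVelocity by the item's weight and destroys the actor.
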(event OnComponentBeginOverlap(PaperSprite)
  (params (OverlappedComponent :type Primitive%20Component%20Object%20Reference) (OtherActor :type Actor%20Object%20Reference) (OtherComp :type Primitive%20Component%20Object%20Reference) (OtherBodyIndex :type Integer) (bFromSweep :type Boolean) (SweepResult :type Hit%20Result%20Structure%20%28by%20ref%29))
  (Utilities|FlowControl|DoOnce false
    (:Completed
      (bind _asbp_character (Utilities|Casting|CastToBP_Character (Game|GetPlayerCharacter 0)))
      (Variables|/Game/Blueprints/BP_Character.BP_Character_C|SetCanMove _asbp_character false)
      (CallFunction|PlayAnimation))))

(event Custom|PlayAnimation
  (Variables|Default|SetFromPosition (Transformation|GetActorLocation))
  (Variables|Default|SetGameTimeAtAnimStart (Utilities|Time|GetGameTimeinSeconds))
  (bind _bottomtotop (Timeline|CollectBottomToTop Play)
    (:Update
      (Transformation|SetActorLocation (Math|Vector|Lerp(Vector) (Variables|Default|GetFromPosition) (+ (Transformation|GetActorLocation (Game|GetPlayerCharacter 0)) "0.000000,0.000000,100.000000") _bottomtotop) false false))
    (:Finished
      (Variables|Default|SetFromPosition (Transformation|GetActorLocation))
      (Utilities|FlowControl|Delay 0.5)
      (bind _toptoplayer (Timeline|CollectTopToPlayer Play)
        (:Update
          (Transformation|SetActorLocation (Math|Vector|Lerp(Vector) (Variables|Default|GetFromPosition) (Transformation|GetActorLocation (Game|GetPlayerCharacter 0)) _toptoplayer) false false))
        (:Finished
          (bind _asbp_character (Utilities|Casting|CastToBP_Character (Game|GetPlayerCharacter 0)))
          (Variables|/Game/Blueprints/BP_Character.BP_Character_C|SetCanMove _asbp_character true)
          (CallFunction|EquipItem))))))

(event EventBeginPlay
  (Variables|Default|SetUniqueItemLocation (Transformation|GetActorLocation)))

(event EventTick
  (params (DeltaSeconds :type Float%20%28single-precision%29)))

(event EventInteract
  (Utilities|FlowControl|DoOnce false
    (:Completed
      (CallFunction|Collect))))

(fn ConstructionScript)

(fn Collect
  (bind _asbp_character (Utilities|Casting|CastToBP_Character (Game|GetPlayerCharacter 0)))
  (Variables|/Game/Blueprints/BP_Character.BP_Character_C|SetCanMove _asbp_character false)
  (CallFunction|PlayAnimation))

(fn EquipItem
  (bind _asbp_character (Utilities|Casting|CastToBP_Character (Game|GetPlayerCharacter 0)))
  (bind _returnvalue (AddComponent|AddPaperSpriteComponent _asbp_character false (Math|Transform|MakeTransform (Variables|Default|GetOffsetEquipItem))))
  (Rendering|Components|Sprite|SetSprite _returnvalue (Sprite|GetSprite (Variables|Default|GetPaperSprite)))
  (Variables|/Script/Engine.CharacterMovementComponent|SetJumpZVelocity (Variables|/Script/Engine.Character|GetCharacterMovement _asbp_character) (- (Variables|/Script/Engine.CharacterMovementComponent|GetJumpZVelocity (Variables|/Script/Engine.Character|GetCharacterMovement _asbp_character)) (Variables|Default|GetWeigthOnJumpVelocity)))
  (Actor|DestroyActor))