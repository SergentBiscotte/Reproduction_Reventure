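; Interactable Paper2D chest that opens once and spawns the sword, shield or shovel collectible selected by ItemContained at its own transform.
; While closed, its detection box shows or hides the character's exclamation-point flipbook on overlap.
; Interact runs through a DoOnce into OpenChest, which hides the prompt and, if SpriteAfterInteract is valid, swaps the sprite and sets IsOpen.
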(event OnComponentBeginOverlap(BoxDetection)
  (params (OverlappedComponent :type Primitive%20Component%20Object%20Reference) (OtherActor :type Actor%20Object%20Reference) (OtherComp :type Primitive%20Component%20Object%20Reference) (OtherBodyIndex :type Integer) (bFromSweep :type Boolean) (SweepResult :type Hit%20Result%20Structure%20%28by%20ref%29))
  (if (not (Variables|Default|GetIsOpen))
    (bind _asbp_character (Utilities|Casting|CastToBP_Character OtherActor))
    (CallFunction|ShowExclamationPoint _asbp_character true)))

(event OnComponentEndOverlap(BoxDetection)
  (params (OverlappedComponent :type Primitive%20Component%20Object%20Reference) (OtherActor :type Actor%20Object%20Reference) (OtherComp :type Primitive%20Component%20Object%20Reference) (OtherBodyIndex :type Integer))
  (if (not (Variables|Default|GetIsOpen))
    (bind _asbp_character (Utilities|Casting|CastToBP_Character OtherActor))
    (CallFunction|ShowExclamationPoint _asbp_character false)))

(event EventBeginPlay)

(event Collision|EventActorBeginOverlap
  (params (OtherActor :type Actor%20Object%20Reference)))

(event EventTick
  (params (DeltaSeconds :type Float%20%28single-precision%29)))

(event EventInteract
  (bind _returnvalue (Transformation|GetActorTransform))
  (Utilities|FlowControl|DoOnce false
    (:Completed
      (CallFunction|OpenChest)
      (switch Utilities|FlowControl|Switch|SwitchonEnum_CollectibleType (Variables|Default|GetItemContained)
        (:NewEnumerator0
          (Game|SpawnActorfromClass "/Game/Blueprints/Interactables/Collectibles/BP_Collectible_Sword.BP_Collectible_Sword_C" _returnvalue "Undefined" 0 0))
        (:NewEnumerator1
          (Game|SpawnActorfromClass "/Game/Blueprints/Interactables/Collectibles/BP_Collectible_Shield.BP_Collectible_Shield_C" _returnvalue "Undefined" 0 0))
        (:NewEnumerator2
          (Game|SpawnActorfromClass "/Game/Blueprints/Interactables/Collectibles/BP_Collectible_Shovel.BP_Collectible_Shovel_C" _returnvalue "Undefined" 0 0))))))

(fn ConstructionScript)

(fn OpenChest
  (bind _spriteafterinteract (Variables|Default|GetSpriteAfterInteract))
  (if (not (Variables|Default|GetIsOpen))
    (bind _asbp_character (Utilities|Casting|CastToBP_Character (Game|Player|GetPlayerPawn 0)))
    (CallFunction|ShowExclamationPoint _asbp_character false)
    (Utilities|IsValid _spriteafterinteract
      (:Is%20Valid
        (Rendering|Components|Sprite|SetSprite (Variables|Default|GetPaperSprite) _spriteafterinteract)
        (Variables|Default|SetIsOpen true)))))

(fn ShowExclamationPoint
  (params (player :type BP%20Character%20Object%20Reference) (show :type Boolean))
  (Development|SetHiddeninGame (Variables|/Game/Blueprints/BP_Character.BP_Character_C|GetExclamationPoint player) (not show) false)
  (Components|Timeline|SetLooping (Variables|/Game/Blueprints/BP_Character.BP_Character_C|GetExclamationPoint player) false)
  (Components|Timeline|PlayfromStart (Variables|/Game/Blueprints/BP_Character.BP_Character_C|GetExclamationPoint player)))