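; Game instance for a Reventure game that holds the endings table, player name substitution, in-game calendar and ending unlock progress.
; Init fills EndTab with five written French endings (text, map, picture, elapsed time, video assets) and placeholders up to 100.
; UnlockNewEnd records the reached ending, advances the year and day counters, then either flags it as already unlocked or unlocks it and increments the completed count.
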(event EventInit
  (CallFunction|InitEndTab))

(fn InitEndTab
  (Utilities|FlowControl|Sequence
    (:then_0
      (Utilities|Array|Add (Variables|Default|GetEndTab) (Utilities|Struct|MakeSTR_End 1 "Il est dangereux d'être proche de {0}" "{0} avait tellement envie d'essayer sa nouvelle épée qu'il ne pu attendre de trouver un sbire, alors il planta l'Ancien du village, juste à côté. 
Et il a volé sa bourse aussi, quelle enflure !" "Ne pas écouter les vieux" "LVL_End_1" "/Game/Assets/EndPicture/Reventure_End1_Picture.Reventure_End1_Picture" 4 0 "{0}] passa pas mal de temps en prison pour ce meurtre. Après avoir été relâché, il s'est dit qu'il devrait peut-être changer de nom, maintenant que c'était une option dans le menu. Histoire d'améliorer son image, m'voyez." "4 ans plus tard..." false "/Game/Assets/EndVideo/MP_Reventure_Ending_1.MP_Reventure_Ending_1" "/Game/Assets/EndVideo/Reventure_Ending_1.Reventure_Ending_1" "/Game/Assets/EndVideo/M_Reventure_Ending_1.M_Reventure_Ending_1")))
    (:then_1
      (Utilities|Array|Add (Variables|Default|GetEndTab) (Utilities|Struct|MakeSTR_End 2 "Je suis stagiaire, j'ai le droit à l'erreur non ? Ah ok pardon..." "Ce jour-là, {0} se prit les pieds dans le caillou à la sortie de sa maison et tomba face la première. 
Le garde juste à côté se demanda si c'était vraiment le héros dont le royaume avait besoin." "Attention à la marche" "LVL_End_1" "/Game/Assets/EndPicture/Reventure_End2_Picture.Reventure_End2_Picture" 0 0 "Quelle chute stupide. Le visage de Tim avait l'air plus plat qu'avant, et c'est dire, vu qu'il était déjà très pixelisé. Il fera attention la prochaine fois qu'il sortira de la maison." "Le même jour ..." false "/Game/Assets/EndVideo/MP_Reventure_Ending_2.MP_Reventure_Ending_2" "/Game/Assets/EndVideo/Reventure_Ending_2.Reventure_Ending_2" "/Game/Assets/EndVideo/M_Reventure_Ending_2.M_Reventure_Ending_2")))
    (:then_2
      (Utilities|Array|Add (Variables|Default|GetEndTab) (Utilities|Struct|MakeSTR_End 3 "Petit mais costaud !" "{0} s'attendait à ce que ces petits sbires soient inoffensifs, ou qu'ils ne prennent qu'un seul coeur de sa vie... 
Et bien c'est exactement ce qu'ils ont fait : Ils ont pris le dernier coeur de sa vie. Le petit et faible coeur de {0}" "Mignonnes petites épées" "LVL_End_1" "/Game/Assets/EndPicture/Reventure_End3_Picture.Reventure_End3_Picture" 0 4 "Tout le monde savait que Tim était un bâtard sans coeur, alors la plaie n'était pas si mal pour lui. Mais bon, il voit un intérêt au bouclier maintenant..." "4 jours plus tard" false "/Game/Assets/EndVideo/MP_Reventure_Ending_3.MP_Reventure_Ending_3" "/Game/Assets/EndVideo/Reventure_Ending_3.Reventure_Ending_3" "/Game/Assets/EndVideo/M_Reventure_Ending_3.M_Reventure_Ending_3")))
    (:then_3
      (Utilities|Array|Add (Variables|Default|GetEndTab) (Utilities|Struct|MakeSTR_End 4 "Ennemi public !" "{0} retira l'épée de Légende du rocher juste pour la planter dans un garde amical. 
Il fut arrêté, et exécuté publiquement pour les charges de \"être un enfoiré.\"" "Défier l'autorité" "LVL_End_1" "/Game/Assets/EndPicture/Reventure_End4_Picture.Reventure_End4_Picture" 0 6 "{0} était un taré, et n'a eu que ce qu'il méritait. Le jour après son exécution, son frère décida de reprendre là où ça en était, et d'accomplir la prophétie..." "6 jours plus tard..." false "/Game/Assets/EndVideo/MP_Reventure_Ending_4.MP_Reventure_Ending_4" "/Game/Assets/EndVideo/Reventure_Ending_4.Reventure_Ending_4" "/Game/Assets/EndVideo/M_Reventure_Ending_4.M_Reventure_Ending_4")))
    (:then_4
      (Utilities|Array|Add (Variables|Default|GetEndTab) (Utilities|Struct|MakeSTR_End 5 "Le Régicide !" "Vive le roi {0} Jr. ! 
Avec la mort du roi précédent, le royaume allait entrer dans une ère de prospérité... 
plutôt brève, puisque l'idée de {0} Jr. devint très vite populaire." "Le jeu du trône" "LVL_End_1" "/Game/Assets/EndPicture/Reventure_End5_Picture.Reventure_End5_Picture" 2 0 "{0} \"le Bref\" fini par se remettre des blessures laissées par la tentative d'assassinat sur sa royale personne. Pour rester en vie, il jura loyauté au nouveauté roi, humilié." "2 ans plus tard..." false "/Game/Assets/EndVideo/MP_Reventure_Ending_5.MP_Reventure_Ending_5" "/Game/Assets/EndVideo/Reventure_Ending_5.Reventure_Ending_5" "/Game/Assets/EndVideo/M_Reventure_Ending_5.M_Reventure_Ending_5")))
    (:then_5
      (for _index (range 6 100)
        (Utilities|Array|Add (Variables|Default|GetEndTab) (Utilities|Struct|MakeSTR_End _index "TITRE A REMPLACER" "DESCRIPTION A REMPLACER" "INDICE A REMPLACER" "None" "/Game/Assets/Images/Reventure_BackgroundPattern.Reventure_BackgroundPattern" 1 3 "TEXTE A REMPLACER" "TEXTE A REMPLACER" false "/Game/Assets/EndVideo/MP_Reventure_Ending_1.MP_Reventure_Ending_1" "/Game/Assets/EndVideo/Reventure_Ending_1.Reventure_Ending_1" "/Game/Assets/EndVideo/M_Reventure_Ending_1.M_Reventure_Ending_1"))))))

(fn ReplacePlayerName
  (params (text :type String))
  (return (Utilities|String|Replace (Utilities|String|Replace text "{0}" (Utilities|String|ToString(Name) (Variables|Default|GetactualPlayerName))) "<br>" " 
")))

(fn AddYearDay
  (params (year :type Integer) (day :type Integer))
  (Variables|Default|SetactualYear (+ (Variables|Default|GetactualYear) year))
  (Variables|Default|SetactualDay (+ (Variables|Default|GetactualDay) day)))

(fn UnlockNewEnd
  (params (numberEnd :type Integer))
  (Variables|Default|SetisAlreadyUnlockEnd false)
  (Variables|Default|SetisJustLookingOldEnd false)
  (Variables|Default|SetisUnlockingNewEnd false)
  (bind _end (CallFunction|GetEndbyNumber numberEnd (Variables|Default|GetEndTab)))
  (bind _output_get (LocalVariables|SetactualEnd _end))
  (Variables|Default|SetlastEnd (LocalVariables|GetactualEnd))
  (CallFunction|AddYearDay (.year _output_get) (.day _output_get))
  (if (.isunlock _output_get)
    (Variables|Default|SetisAlreadyUnlockEnd true)
    (else
      (CallFunction|SetEndbyNumber (Variables|Default|GetEndTab) (Utilities|Struct|MakeSTR_End (.number (LocalVariables|GetactualEnd)) (.titre (LocalVariables|GetactualEnd)) (.description (LocalVariables|GetactualEnd)) (.clue (LocalVariables|GetactualEnd)) (.mapendname (LocalVariables|GetactualEnd)) (.endpicture (LocalVariables|GetactualEnd)) (.year (LocalVariables|GetactualEnd)) (.day (LocalVariables|GetactualEnd)) (.newdaytext (LocalVariables|GetactualEnd)) (.newdayloadingtext (LocalVariables|GetactualEnd)) true (.mediaplayer (LocalVariables|GetactualEnd)) (.videosource (LocalVariables|GetactualEnd)) (.videomaterial (LocalVariables|GetactualEnd))))
      (Variables|Default|SetisUnlockingNewEnd true)
      (Variables|Default|SetNumberAccomplishedEnd (+ (Variables|Default|GetNumberAccomplishedEnd) 1)))))