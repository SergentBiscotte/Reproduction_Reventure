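; BP_EnemyMinion is a 2D flipbook enemy that patrols along X between two checkpoint offsets from its spawn location.
; Tick drives movement, reverses at each checkpoint by mirroring the sprite's X scale, and picks the walk or attack flipbook.
; Hitting BP_Character's capsule deals damage and briefly flags attacking, with a DoOnce and delay as cooldown.
; EnemyAttacked destroys it immediately; the turn-on-obstacle logic is unconnected.
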(event OnComponentHit(CapsuleComponent)
  (params (HitComponent :type Primitive%20Component%20Object%20Reference) (OtherActor :type Actor%20Object%20Reference) (OtherComp :type Primitive%20Component%20Object%20Reference) (NormalImpulse :type Vector :default "0, 0, 0") (Hit :type Hit%20Result%20Structure%20%28by%20ref%29))
  (bind _asbp_character (Utilities|Casting|CastToBP_Character OtherActor))
  (if (== (Variables|/Script/Engine.Character|GetCapsuleComponent _asbp_character) OtherComp)
    ;[1 0.5481 0.09168] Testing atk
    (Utilities|FlowControl|DoOnce false :!label _label
      (:Completed
        (Variables|Default|SetIs%20Attacking true)
        (Default|TakeDamage _asbp_character)
        (Utilities|FlowControl|Sequence
          (:then_0
            (Utilities|FlowControl|Delay 0.5)
            (Variables|Default|SetIs%20Attacking false))
          (:then_1
            (Utilities|FlowControl|Delay (Variables|Default|GetDelayBetweenAttack))
            (goto _label Reset)))))))

(event Custom|EnemyAttacked
  (CallFunction|Death))

(event EventBeginPlay
  ;[0.05124 1 0.1642] Change side of sprite if going right or left
  (CallFunction|UpdateAnimation)
  (CallFunction|ToggleDirection)
  (Variables|Default|SetOriginalXLocation (.x (Transformation|GetActorLocation))))

(event EventTick
  (params (DeltaSeconds :type Float%20%28single-precision%29))
  ;[0 1 0.004695] Moving enemy
  (Variables|/Script/Engine.CharacterMovementComponent|SetMaxWalkSpeed (Variables|Character|GetCharacterMovement) (Variables|Default|GetWalkSpeed))
  (Pawn|Input|AddMovementInput "1.000000,0.000000,0.000000" (select (Variables|Default|GetMoveRight) 1.0 -1.0) false)
  (CallFunction|UpdateAnimation)
  (if (or (and (not (Variables|Default|GetMoveRight)) (Math|Float|NearlyEqual(Float) (.x (Transformation|GetActorLocation)) (+ (.x (Variables|Default|GetCheckpoint1)) (Variables|Default|GetOriginalXLocation)) 2.0)) (and (Math|Float|NearlyEqual(Float) (.x (Transformation|GetActorLocation)) (+ (.x (Variables|Default|GetCheckpoint2)) (Variables|Default|GetOriginalXLocation)) 2.0) (Variables|Default|GetMoveRight)))
    (Variables|Default|SetMoveRight (not (Variables|Default|GetMoveRight)))
    (CallFunction|ToggleDirection)))

(fn ConstructionScript)

(fn Death
  (Actor|DestroyActor))

(fn ToggleDirection
  (bind _sprite (Variables|Default|GetSprite))
  (bind _returnvalue (Transformation|GetWorldScale _sprite))
  (Transformation|SetWorldScale3D (Variables|Default|GetSprite) (Math|Vector|MakeVector (* (Math|Float|Absolute(Float) (.x _returnvalue)) (select (Variables|Default|GetMoveRight) 1.0 -1.0)) (.y _returnvalue) (.z _returnvalue))))

(fn AttackPlayer
  (Sprite|SetFlipbook (Variables|Default|GetSprite) (Variables|Default|GetAttackFlipbook)))

(fn UpdateAnimation
  (Sprite|SetFlipbook (Variables|Default|GetSprite) (select (Variables|Default|GetIs%20Attacking) (Variables|Default|GetAttackFlipbook) (select (Variables|Default|GetIs%20Dead) 0 (Variables|Default|GetWalk)))))