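; Player controller that routes in-game key, gamepad and mouse input to GM_Game and its pause menu.
; Any key becomes widget navigation once the start day has finished; before that it answers the game mode's wait-for-button state.
; Escape, M or gamepad Special Right toggle pause outside cinematic mode.
; While paused, confirm keys and left click trigger pause menu buttons, and a widget click event plays a sound then follows the click path.
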(event Custom|EventWidgetClickOnButton_Event
  (Audio|PlaySound2D "/Game/Assets/Test/CMPTKey_Souris_raspberry_simple_clic__ID_1735__LS_Cue.CMPTKey_Souris_raspberry_simple_clic__ID_1735__LS_Cue" 1.0 1.0 0.0 0 0)
  (bind _asgm_game (Utilities|Casting|CastToGM_Game (Game|GetGameMode)))
  (if (Variables|/Game/Blueprints/GameModes/GM_Game.GM_Game_C|GetisGamePaused _asgm_game)
    (Default|LeftMouseClickButton (Variables|/Game/Blueprints/GameModes/GM_Game.GM_Game_C|GetwPauseMenuRef _asgm_game))))

(event EventBeginPlay)

(event EventTick
  (params (DeltaSeconds :type Float%20%28single-precision%29)))

(event Input|KeyboardEvents|Enter
  (params (Key :type Key%20Structure :default "None"))
  (:Pressed
    (bind _asgm_game (Utilities|Casting|CastToGM_Game (Game|GetGameMode)))
    (if (Variables|/Game/Blueprints/GameModes/GM_Game.GM_Game_C|GetisGamePaused _asgm_game)
      (Default|ActionButton (Variables|/Game/Blueprints/GameModes/GM_Game.GM_Game_C|GetwPauseMenuRef _asgm_game)))))

(event Input|GamepadEvents|GamepadSpecialRight
  (params (Key :type Key%20Structure :default "None"))
  (:Pressed
    (bind _asbp_character (Utilities|Casting|CastToBP_Character (Game|Player|GetPlayerPawn 0)))
    (if (not (Variables|/Game/Blueprints/BP_Character.BP_Character_C|GetisInCinematicMode _asbp_character))
      (bind _asgm_game (Utilities|Casting|CastToGM_Game (Game|GetGameMode)))
      (Default|SetPause _asgm_game (not (Variables|/Game/Blueprints/GameModes/GM_Game.GM_Game_C|GetisGamePaused _asgm_game))))))

(event Input|KeyboardEvents|AnyKey
  (params (Key :type Key%20Structure :default "None"))
  (:Pressed
    (bind _asgm_game (Utilities|Casting|CastToGM_Game (Game|GetGameMode)))
    (if (Variables|/Game/Blueprints/GameModes/GM_Game.GM_Game_C|GetisStartDayFinished _asgm_game)
      (bind _enum (CallFunction|TranslateKeytoWidgetNavigation Key))
      (Default|NavigationWidget _asgm_game _enum)
      (elif (Variables|/Game/Blueprints/GameModes/GM_Game.GM_Game_C|GetisButtonPressedWaiting _asgm_game)
        (Default|PressedButton _asgm_game)))))

(event Input|GamepadEvents|GamepadFaceButtonBottom
  (params (Key :type Key%20Structure :default "None"))
  (:Pressed
    (bind _asgm_game (Utilities|Casting|CastToGM_Game (Game|GetGameMode)))
    (if (Variables|/Game/Blueprints/GameModes/GM_Game.GM_Game_C|GetisGamePaused _asgm_game)
      (Default|ActionButton (Variables|/Game/Blueprints/GameModes/GM_Game.GM_Game_C|GetwPauseMenuRef _asgm_game)))))

(event Input|KeyboardEvents|Escape
  (params (Key :type Key%20Structure :default "None"))
  (:Pressed
    (bind _asbp_character (Utilities|Casting|CastToBP_Character (Game|Player|GetPlayerPawn 0)))
    (if (not (Variables|/Game/Blueprints/BP_Character.BP_Character_C|GetisInCinematicMode _asbp_character))
      (bind _asgm_game (Utilities|Casting|CastToGM_Game (Game|GetGameMode)))
      (Default|SetPause _asgm_game (not (Variables|/Game/Blueprints/GameModes/GM_Game.GM_Game_C|GetisGamePaused _asgm_game))))))

(event Input|MouseEvents|LeftMouseButton
  (params (Key :type Key%20Structure :default "None"))
  (:Pressed
    (bind _asgm_game (Utilities|Casting|CastToGM_Game (Game|GetGameMode)))
    (if (Variables|/Game/Blueprints/GameModes/GM_Game.GM_Game_C|GetisGamePaused _asgm_game)
      (Default|LeftMouseClickButton (Variables|/Game/Blueprints/GameModes/GM_Game.GM_Game_C|GetwPauseMenuRef _asgm_game)))))

(event Input|KeyboardEvents|M
  (params (Key :type Key%20Structure :default "None"))
  (:Pressed
    (bind _asbp_character (Utilities|Casting|CastToBP_Character (Game|Player|GetPlayerPawn 0)))
    (if (not (Variables|/Game/Blueprints/BP_Character.BP_Character_C|GetisInCinematicMode _asbp_character))
      (bind _asgm_game (Utilities|Casting|CastToGM_Game (Game|GetGameMode)))
      (Default|SetPause _asgm_game (not (Variables|/Game/Blueprints/GameModes/GM_Game.GM_Game_C|GetisGamePaused _asgm_game))))))

(event Input|KeyboardEvents|J
  (params (Key :type Key%20Structure :default "None")))

(fn ConstructionScript)