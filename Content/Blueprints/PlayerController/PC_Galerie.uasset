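; Player controller for the gallery menu, turning keyboard, gamepad and mouse presses into menu actions through GM_Menu_Galerie.
; Escape or gamepad right opens the level menu, any key is translated for widget navigation, and Enter, gamepad bottom or left click trigger the gallery widget's actions.
; All input is ignored while a new ending is unlocking; a widget-click event plays a sound and reuses the left-click path.
; Key bindings are hardcoded, marked for Enhanced Input replacement.
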(event Custom|EventWidgetClickOnButton_Event
  (Audio|PlaySound2D "/Game/Assets/Test/CMPTKey_Souris_raspberry_simple_clic__ID_1735__LS_Cue.CMPTKey_Souris_raspberry_simple_clic__ID_1735__LS_Cue" 1.0 1.0 0.0 0 0)
  ;[1 1 1] A REMPLACER PAR DES ENHANCED INPUT
  (bind _asgm_menu_galerie (Utilities|Casting|CastToGM_Menu_Galerie (Game|GetGameMode)))
  (if (not (Variables|/Game/Blueprints/GameModes/GM_Menu_Galerie.GM_Menu_Galerie_C|GetisUnlockingNewEnd _asgm_menu_galerie))
    (Default|LeftMouseClickButton (Variables|/Game/Blueprints/GameModes/GM_Menu_Galerie.GM_Menu_Galerie_C|GetmenuGalerieRef _asgm_menu_galerie))))

(event EventBeginPlay)

(event EventTick
  (params (DeltaSeconds :type Float%20%28single-precision%29)))

(event Input|KeyboardEvents|Enter
  (params (Key :type Key%20Structure :default "None"))
  ;[1 1 1] A REMPLACER PAR DES ENHANCED INPUT
  (:Pressed
    (bind _asgm_menu_galerie (Utilities|Casting|CastToGM_Menu_Galerie (Game|GetGameMode)))
    (if (not (Variables|/Game/Blueprints/GameModes/GM_Menu_Galerie.GM_Menu_Galerie_C|GetisUnlockingNewEnd _asgm_menu_galerie))
      (Default|ActionButton (Variables|/Game/Blueprints/GameModes/GM_Menu_Galerie.GM_Menu_Galerie_C|GetmenuGalerieRef _asgm_menu_galerie)))))

(event Input|KeyboardEvents|Escape
  (params (Key :type Key%20Structure :default "None"))
  ;[1 1 1] A REMPLACER PAR DES ENHANCED INPUT
  (:Pressed
    (bind _asgm_menu_galerie (Utilities|Casting|CastToGM_Menu_Galerie (Game|GetGameMode)))
    (if (not (Variables|/Game/Blueprints/GameModes/GM_Menu_Galerie.GM_Menu_Galerie_C|GetisUnlockingNewEnd _asgm_menu_galerie))
      (Default|OpenLevelMenu _asgm_menu_galerie))))

(event Input|KeyboardEvents|AnyKey
  (params (Key :type Key%20Structure :default "None"))
  ;[1 1 1] A REMPLACER PAR DES ENHANCED INPUT
  (:Pressed
    (bind _enum (CallFunction|TranslateKeytoWidgetNavigation Key))
    (bind _asgm_menu_galerie (Utilities|Casting|CastToGM_Menu_Galerie (Game|GetGameMode)))
    (if (not (Variables|/Game/Blueprints/GameModes/GM_Menu_Galerie.GM_Menu_Galerie_C|GetisUnlockingNewEnd _asgm_menu_galerie))
      (Default|NavigationWidget _asgm_menu_galerie _enum))))

(event Input|GamepadEvents|GamepadFaceButtonBottom
  (params (Key :type Key%20Structure :default "None"))
  ;[1 1 1] A REMPLACER PAR DES ENHANCED INPUT
  (:Pressed
    (bind _asgm_menu_galerie (Utilities|Casting|CastToGM_Menu_Galerie (Game|GetGameMode)))
    (if (not (Variables|/Game/Blueprints/GameModes/GM_Menu_Galerie.GM_Menu_Galerie_C|GetisUnlockingNewEnd _asgm_menu_galerie))
      (Default|ActionButton (Variables|/Game/Blueprints/GameModes/GM_Menu_Galerie.GM_Menu_Galerie_C|GetmenuGalerieRef _asgm_menu_galerie)))))

(event Input|GamepadEvents|GamepadFaceButtonRight
  (params (Key :type Key%20Structure :default "None"))
  ;[1 1 1] A REMPLACER PAR DES ENHANCED INPUT
  (:Pressed
    (bind _asgm_menu_galerie (Utilities|Casting|CastToGM_Menu_Galerie (Game|GetGameMode)))
    (if (not (Variables|/Game/Blueprints/GameModes/GM_Menu_Galerie.GM_Menu_Galerie_C|GetisUnlockingNewEnd _asgm_menu_galerie))
      (Default|OpenLevelMenu _asgm_menu_galerie))))

(event Input|MouseEvents|LeftMouseButton
  (params (Key :type Key%20Structure :default "None"))
  ;[1 1 1] A REMPLACER PAR DES ENHANCED INPUT
  (:Pressed
    (bind _asgm_menu_galerie (Utilities|Casting|CastToGM_Menu_Galerie (Game|GetGameMode)))
    (if (not (Variables|/Game/Blueprints/GameModes/GM_Menu_Galerie.GM_Menu_Galerie_C|GetisUnlockingNewEnd _asgm_menu_galerie))
      (Default|LeftMouseClickButton (Variables|/Game/Blueprints/GameModes/GM_Menu_Galerie.GM_Menu_Galerie_C|GetmenuGalerieRef _asgm_menu_galerie)))))

(fn ConstructionScript)