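; Main menu player controller that turns key presses into calls on the menu game modes.
; Any key whose display name differs from the EchapKeyException string plays a click sound and calls NextLevel on GM_Menu.
; Escape press and release pass true and false to HoldEscape on GM_Menu_MainMenu, leaving the hold logic to that game mode.
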(event EventBeginPlay)

(event EventTick
  (params (DeltaSeconds :type Float%20%28single-precision%29)))

(event Input|KeyboardEvents|AnyKey
  (params (Key :type Key%20Structure :default "None"))
  (:Pressed
    (if (Utilities|Enum|NotEqual(Enum) (Utilities|String|ToString(Text) (Class|KismetInputLibrary|KeyGetDisplayName Key true)) (Variables|Default|GetechapKeyException))
      (Audio|PlaySound2D "/Game/Assets/Test/CMPTKey_Souris_raspberry_simple_clic__ID_1735__LS_Cue.CMPTKey_Souris_raspberry_simple_clic__ID_1735__LS_Cue" 1.0 1.0 0.0 0 0)
      (bind _asgm_menu (Utilities|Casting|CastToGM_Menu (Game|GetGameMode)))
      (Default|NextLevel _asgm_menu))))

(event Input|KeyboardEvents|Escape
  (params (Key :type Key%20Structure :default "None"))
  (:Pressed
    (bind _asgm_menu_main_menu (Utilities|Casting|CastToGM_Menu_MainMenu (Game|GetGameMode)))
    (Default|HoldEscape _asgm_menu_main_menu true))
  (:Released
    (bind _asgm_menu_main_menu_2 (Utilities|Casting|CastToGM_Menu_MainMenu (Game|GetGameMode)))
    (Default|HoldEscape _asgm_menu_main_menu_2 false)))

(fn ConstructionScript)