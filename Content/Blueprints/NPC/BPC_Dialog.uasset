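; NPC dialog component that owns a W_DialogBox widget and shows or hides it with an open animation.
; On BeginPlay it creates the widget, fills in its message and portrait image, and passes the text through GI_GameInfo to substitute the player's name.
; OpenDialog adds the widget to the viewport and plays the animation forward.
; CloseDialog plays it in reverse, binding the animation-finished event to remove the widget.
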(event Custom|RemoveFromViewport
  (bind _wdialogref (Variables|Default|GetwDialogRef))
  (Class|UserWidget|UnbindAllfromAnimationFinished _wdialogref (Variables|/Game/UI/W_DialogBox.W_DialogBox_C|GetOpenDialog _wdialogref))
  (Widget|RemovefromParent (Variables|Default|GetwDialogRef)))

(event EventBeginPlay
  (bind _returnvalue (UserInterface|CreateWidget "/Game/UI/W_DialogBox.W_DialogBox_C"))
  (Variables|Default|SetwDialogRef _returnvalue)
  (CallFunction|SetDialog (Variables|Default|GetMessageDialog))
  (Default|SetImagePDP (Variables|Default|GetwDialogRef) (Variables|Default|GetImagePDP)))

(event EventTick
  (params (DeltaSeconds :type Float%20%28single-precision%29)))

(fn OpenDialog
  (UserInterface|Viewport|AddtoViewport (Variables|Default|GetwDialogRef) 0)
  (Default|PlayOpenAnimation (Variables|Default|GetwDialogRef) "Forward"))

(fn CloseDialog
  (bind _wdialogref (Variables|Default|GetwDialogRef))
  (Class|UserWidget|BindtoAnimationFinished _wdialogref (Variables|/Game/UI/W_DialogBox.W_DialogBox_C|GetOpenDialog _wdialogref) (EventDispatchers|CreateEvent :!event Custom|RemoveFromViewport))
  (Default|PlayOpenAnimation (Variables|Default|GetwDialogRef) "Reverse"))

(fn SetDialog
  (params (Message :type String))
  (bind _asgi_game_info (Utilities|Casting|CastToGI_GameInfo (Game|GetGameInstance)))
  (bind _newtext (Default|ReplacePlayerName _asgi_game_info Message))
  (Default|SetMessageDialog (Variables|Default|GetwDialogRef) _newtext))