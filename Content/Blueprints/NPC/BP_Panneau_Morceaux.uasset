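; BP_Panneau_Morceaux is a 2D wooden sign that shows a dialog when the player character is near it.
; Overlap events on BoxDialog check for BP_Character, then open the dialog through BPCDialog on enter and close it on exit.
; The construction script uses IsRight to pick the right or left "Morceaux" Paper2D flipbook for the sign.
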(event OnComponentBeginOverlap(BoxDialog)
  (params (OverlappedComponent :type Primitive%20Component%20Object%20Reference) (OtherActor :type Actor%20Object%20Reference) (OtherComp :type Primitive%20Component%20Object%20Reference) (OtherBodyIndex :type Integer) (bFromSweep :type Boolean) (SweepResult :type Hit%20Result%20Structure%20%28by%20ref%29))
  (Utilities|Casting|CastToBP_Character OtherActor)
  (Default|OpenDialog (Variables|Default|GetBPC_Dialog)))

(event OnComponentEndOverlap(BoxDialog)
  (params (OverlappedComponent :type Primitive%20Component%20Object%20Reference) (OtherActor :type Actor%20Object%20Reference) (OtherComp :type Primitive%20Component%20Object%20Reference) (OtherBodyIndex :type Integer))
  (Utilities|Casting|CastToBP_Character OtherActor)
  (Default|CloseDialog (Variables|Default|GetBPC_Dialog)))

(event EventBeginPlay)

(event Collision|EventActorBeginOverlap
  (params (OtherActor :type Actor%20Object%20Reference)))

(event EventTick
  (params (DeltaSeconds :type Float%20%28single-precision%29)))

(fn ConstructionScript
  (if (Variables|Default|GetisRight)
    (Sprite|SetFlipbook (Variables|Default|GetPaperFlipbook) "/Game/Assets/Props/Panneau/FB_PanneauWood_MorceauxRight.FB_PanneauWood_MorceauxRight")
    (else
      (Sprite|SetFlipbook (Variables|Default|GetPaperFlipbook) "/Game/Assets/Props/Panneau/FB_PanneauWood_MorceauxLeft.FB_PanneauWood_MorceauxLeft"))))