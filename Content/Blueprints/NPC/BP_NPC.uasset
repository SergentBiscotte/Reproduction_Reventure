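; BP_NPC is a sprite-based NPC that opens a dialog when the player character overlaps its detection box and can die once.
; The box extent is set at construction, and its overlaps drive the BPCDialog component while the NPC is alive.
; DeathNPC closes the dialog, unlocks a numbered ending through GM_Game and plays a timeline that transforms the sprite.
; AttachSword is an empty stub.
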(event OnComponentBeginOverlap(BoxDetectionDialog)
  (params (OverlappedComponent :type Primitive%20Component%20Object%20Reference) (OtherActor :type Actor%20Object%20Reference) (OtherComp :type Primitive%20Component%20Object%20Reference) (OtherBodyIndex :type Integer) (bFromSweep :type Boolean) (SweepResult :type Hit%20Result%20Structure%20%28by%20ref%29))
  (Utilities|Casting|CastToBP_Character OtherActor)
  (if (not (Variables|Default|GetisDead))
    (Default|OpenDialog (Variables|Default|GetBPC_Dialog))))

(event OnComponentEndOverlap(BoxDetectionDialog)
  (params (OverlappedComponent :type Primitive%20Component%20Object%20Reference) (OtherActor :type Actor%20Object%20Reference) (OtherComp :type Primitive%20Component%20Object%20Reference) (OtherBodyIndex :type Integer))
  (Utilities|Casting|CastToBP_Character OtherActor)
  (if (not (Variables|Default|GetisDead))
    (Default|CloseDialog (Variables|Default|GetBPC_Dialog))))

(event Custom|DeathAnimation
  (bind (_direction _rotation _adjustlocation) (Timeline|DeathRotate Play)
    (:Update
      (Transformation|SetWorldLocationAndRotation (Variables|Default|GetSprite) "0, 0, 0" (Math|Rotator|MakeRotator 0.0 (.y (+ (Variables|Default|GetOrigineLocation) (Math|Vector|MakeVector 0.0 (* _adjustlocation -1e+01) 0.0))) 0.0) false false))
    (:Finished
      (Development|PrintString "Death finished !"))))

(event EventBeginPlay
  (Variables|Default|SetOrigineLocation (Transformation|GetWorldLocation (Variables|Default|GetSprite))))

(fn ConstructionScript
  (Components|Box|SetBoxExtent (Variables|Default|GetBoxDetectionDialog) (Variables|Default|GetScaleBoxDialog) true))

(fn DeathNPC
  (if (not (Variables|Default|GetisDead))
    (Variables|Default|SetisDead true)
    (CallFunction|AttachSword)
    (Default|CloseDialog (Variables|Default|GetBPC_Dialog))
    (bind _asgm_game (Utilities|Casting|CastToGM_Game (Game|GetGameMode)))
    (Default|UnlockNewEndTimer _asgm_game (Variables|Default|GetNumberEnd))
    (CallFunction|DeathAnimation)))

(fn AttachSword)