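; BP_CadrePhoto is a photo frame actor that only stays in the level if a specific game ending has been unlocked.
; On BeginPlay it reads the ending table from GI_GameInfo, looks up the ending at index five and destroys itself if that ending is still locked.
; The construction script applies its Sprite variable to the PaperSprite component.
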(event EventBeginPlay
  (bind _asgi_game_info (Utilities|Casting|CastToGI_GameInfo (Game|GetGameInstance)))
  (bind _end (CallFunction|GetEndbyNumber 5 (Variables|/Game/Blueprints/GameInstance/GI_GameInfo.GI_GameInfo_C|GetEndTab _asgi_game_info)))
  (if (not (.isunlock _end))
    (Actor|DestroyActor self)))

(event Collision|EventActorBeginOverlap
  (params (OtherActor :type Actor%20Object%20Reference)))

(event EventTick
  (params (DeltaSeconds :type Float%20%28single-precision%29)))

(fn ConstructionScript
  (Rendering|Components|Sprite|SetSprite (Variables|Default|GetPaperSprite) (Variables|Default|GetSprite)))