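; Guard NPC Blueprint, a child of a base NPC class, with special handling for an actor tagged as the first guard.
; When that guard dies, the death override records the kill in the game instance.
; On begin play, it reads that flag and either restores the guard as a dead, adjusted flipbook sprite or greatly enlarges its dialog detection box.
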(event EventBeginPlay
  (|CallParentFunction)
  (Variables|Default|SetNumberEnd 4)
  (CallFunction|ExceptionFirstGuard))

(event Collision|EventActorBeginOverlap
  (params (OtherActor :type Actor%20Object%20Reference)))

(event EventTick
  (params (DeltaSeconds :type Float%20%28single-precision%29)))

(fn ConstructionScript
  (|CallParentFunction))

(fn DeathNPC
  (|CallParentFunction)
  (if (> (Utilities|Array|Length (Variables|Default|GetTags)) 0)
    (if (== (Utilities|Array|Get(acopy) (Variables|Default|GetTags)) "FirstGuard")
      (bind _asgi_game_info (Utilities|Casting|CastToGI_GameInfo (Game|GetGameInstance)))
      (Variables|/Game/Blueprints/GameInstance/GI_GameInfo.GI_GameInfo_C|SetisFirstGuardKilled _asgi_game_info true))))

(fn ExceptionFirstGuard
  (bind _sprite (Variables|Default|GetSprite))
  (bind _boxdetectiondialog (Variables|Default|GetBoxDetectionDialog))
  (if (> (Utilities|Array|Length (Variables|Default|GetTags)) 0)
    (if (== (Utilities|Array|Get(acopy) (Variables|Default|GetTags)) "FirstGuard")
      (bind _asgi_game_info (Utilities|Casting|CastToGI_GameInfo (Game|GetGameInstance)))
      (if (Variables|/Game/Blueprints/GameInstance/GI_GameInfo.GI_GameInfo_C|GetisFirstGuardKilled _asgi_game_info)
        (Variables|Default|SetisDead true)
        (Sprite|SetFlipbook _sprite "/Game/Assets/Characters/Guard/FB_Guard_dead.FB_Guard_dead")
        (Transformation|SetRelativeScale3D _sprite "0.500000,0.500000,0.500000")
        (Transformation|SetRelativeLocation _sprite (- (Variables|/Script/Engine.SceneComponent|GetRelativeLocation _sprite) "0.000000,0.000000,2.000000") false false)
        (else
          (Transformation|SetWorldScale3D _boxdetectiondialog (* (Transformation|GetWorldScale _boxdetectiondialog) 7.5)))))))