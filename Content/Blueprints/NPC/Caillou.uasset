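; Caillou is a stone that trips the player into a scripted fall ending, and it only stays in the level once at least four endings have been accomplished.
; On overlap, it disables player movement, gravity and capsule collision, then chains three timelines that lerp the player up, down and along a slide.
; Target points are offset from the stone, mirrored by the player's X velocity and raised by capsule half-height, and the last timeline unlocks an ending through GM_Game.
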(event OnComponentBeginOverlap(BoxDetection)
  (params (OverlappedComponent :type Primitive%20Component%20Object%20Reference) (OtherActor :type Actor%20Object%20Reference) (OtherComp :type Primitive%20Component%20Object%20Reference) (OtherBodyIndex :type Integer) (bFromSweep :type Boolean) (SweepResult :type Hit%20Result%20Structure%20%28by%20ref%29))
  (bind _asbp_character (Utilities|Casting|CastToBP_Character OtherActor))
  (Variables|Default|Setplayer _asbp_character)
  (CallFunction|StartPlayerFall))

(event Custom|MoveFallUp
  (bind _fallup (Timeline|TimelineFallUp Play)
    (:Update
      (Transformation|SetActorLocation (Variables|Default|Getplayer) (Math|Vector|Lerp(Vector) (Variables|Default|GetOriginalPosition) (Variables|Default|GetNewPosition) _fallup) false false))
    (:Finished
      (CallFunction|AssignOriginalPosition (Variables|AnimationPoint|GetFallUpPoint))
      (CallFunction|AssignNewPosition (Variables|AnimationPoint|GetFallDownPoint))
      (CallFunction|MoveFallDown))))

(event Custom|MoveFallDown
  (bind _falldown (Timeline|TimelineFallDown Play)
    (:Update
      (Transformation|SetActorLocation (Variables|Default|Getplayer) (Math|Vector|Lerp(Vector) (Variables|Default|GetOriginalPosition) (Variables|Default|GetNewPosition) _falldown) false false)
      (if (> _falldown 0.5)
        (Utilities|FlowControl|DoOnce false
          (:Completed
            (Variables|/Game/Blueprints/BP_Character.BP_Character_C|SetIsFallingDown (Variables|Default|Getplayer) true)))))
    (:Finished
      (CallFunction|AssignOriginalPosition (Variables|AnimationPoint|GetFallDownPoint))
      (CallFunction|AssignNewPosition (Variables|AnimationPoint|GetSlideDownPoint))
      (CallFunction|MoveSlideDown))))

(event Custom|MoveSlideDown
  (bind _slidedown (Timeline|TimelineSlideDown Play)
    (:Update
      (Transformation|SetActorLocation (Variables|Default|Getplayer) (Math|Vector|Lerp(Vector) (Variables|Default|GetOriginalPosition) (Variables|Default|GetNewPosition) _slidedown) false false))
    (:Finished
      (bind _asgm_game (Utilities|Casting|CastToGM_Game (Game|GetGameMode)))
      (Default|UnlockNewEnd _asgm_game 2))))

(event EventBeginPlay
  (bind _asgi_game_info (Utilities|Casting|CastToGI_GameInfo (Game|GetGameInstance)))
  (if (>= (Variables|/Game/Blueprints/GameInstance/GI_GameInfo.GI_GameInfo_C|GetNumberAccomplishedEnd _asgi_game_info) 4)
    (Collision|SetCollisionEnabled (Variables|Default|GetBoxDetection) "QueryAndPhysics")
    (else
      (Actor|DestroyActor self))))

(event Collision|EventActorBeginOverlap
  (params (OtherActor :type Actor%20Object%20Reference)))

(event EventTick
  (params (DeltaSeconds :type Float%20%28single-precision%29)))

(fn ConstructionScript)

(fn StartPlayerFall
  (bind _player (Variables|Default|Getplayer))
  (Collision|SetCollisionEnabled (Variables|Default|GetBoxDetection) "NoCollision")
  (Variables|/Game/Blueprints/BP_Character.BP_Character_C|SetIsFallingUp (Variables|Default|Getplayer) true)
  (Variables|/Game/Blueprints/BP_Character.BP_Character_C|SetCanMove (Variables|Default|Getplayer) false)
  ;[1 1 1] Différentes valeurs utiles pour déterminer la position lors de l'animation
  (Variables|Default|SetOriginalPosition (Transformation|GetActorLocation))
  (Variables|Default|SetDirectionX (Math|Float|SelectFloat 1.0 -1.0 (> (.X (Math|Vector|BreakVector (Variables|/Script/Engine.MovementComponent|GetVelocity (Variables|/Script/Engine.Character|GetCharacterMovement (Variables|Default|Getplayer))))) 0.0)))
  (Variables|Default|SetDifferenceZ (Components|Capsule|GetScaledCapsuleHalfHeight (Variables|/Script/Engine.Character|GetCapsuleComponent (Variables|Default|Getplayer))))
  (Utilities|FlowControl|Sequence
    (:then_0
      ;[1 1 1] Désactive la physique et le mouvement du joueur
      (Physics|SetSimulatePhysics (Variables|/Script/Engine.Character|GetCapsuleComponent _player) false)
      (Variables|/Script/Engine.CharacterMovementComponent|SetGravityScale (Variables|/Script/Engine.Character|GetCharacterMovement _player) 0.0)
      (Collision|SetCollisionEnabled (Variables|/Script/Engine.Character|GetCapsuleComponent _player) "NoCollision")
      (Pawn|Components|CharacterMovement|DisableMovement (Variables|/Script/Engine.Character|GetCharacterMovement _player)))
    (:then_1
      (CallFunction|AssignNewPosition (Variables|AnimationPoint|GetFallUpPoint))
      (CallFunction|MoveFallUp))))

(fn AssignNewPosition
  (params (animationPoint :type Vector))
  (Variables|Default|SetNewPosition (+ (Transformation|GetActorLocation) (Math|Vector|MakeVector (* (.x animationPoint) (Variables|Default|GetDirectionX)) (.y animationPoint) (+ (.z animationPoint) (Variables|Default|GetDifferenceZ))))))

(fn AssignOriginalPosition
  (params (animationPoint :type Vector))
  (Variables|Default|SetOriginalPosition (Transformation|GetActorLocation (Variables|Default|Getplayer))))