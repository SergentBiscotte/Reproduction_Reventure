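; BP_Panneau is a flipbook sign NPC that shows its dialog while the player character overlaps its box, until broken.
; The construction script picks steel or wood visuals and portrait from IsUnbreakable.
; BreakPanneau swaps wooden signs to a broken flipbook, closes the dialog, and spawns two BP_Panneau_Morceaux pieces toward the player with an impulse, each carrying half the message.
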(event OnComponentBeginOverlap(BoxDialog)
  (params (OverlappedComponent :type Primitive%20Component%20Object%20Reference) (OtherActor :type Actor%20Object%20Reference) (OtherComp :type Primitive%20Component%20Object%20Reference) (OtherBodyIndex :type Integer) (bFromSweep :type Boolean) (SweepResult :type Hit%20Result%20Structure%20%28by%20ref%29))
  (Utilities|Casting|CastToBP_Character OtherActor)
  (if (not (Variables|Default|GetisBroken))
    (Default|OpenDialog (Variables|Default|GetBPC_Dialog))))

(event OnComponentEndOverlap(BoxDialog)
  (params (OverlappedComponent :type Primitive%20Component%20Object%20Reference) (OtherActor :type Actor%20Object%20Reference) (OtherComp :type Primitive%20Component%20Object%20Reference) (OtherBodyIndex :type Integer))
  (Utilities|Casting|CastToBP_Character OtherActor)
  (if (not (Variables|Default|GetisBroken))
    (Default|CloseDialog (Variables|Default|GetBPC_Dialog))))

(event EventBeginPlay)

(event Collision|EventActorBeginOverlap
  (params (OtherActor :type Actor%20Object%20Reference)))

(event EventTick
  (params (DeltaSeconds :type Float%20%28single-precision%29)))

(fn ConstructionScript
  (if (Variables|Default|GetisUnbreakable)
    (Variables|/Game/Blueprints/NPC/BPC_Dialog.BPC_Dialog_C|SetImagePDP (Variables|Default|GetBPC_Dialog) "/Game/Assets/Dialog/Reventure_PDP_PanneauSteel.Reventure_PDP_PanneauSteel")
    (Sprite|SetFlipbook (Variables|Default|GetPaperFlipbook) "/Game/Assets/Props/Panneau/FB_Reventure_PanneauSteel.FB_Reventure_PanneauSteel")
    (else
      (Variables|/Game/Blueprints/NPC/BPC_Dialog.BPC_Dialog_C|SetImagePDP (Variables|Default|GetBPC_Dialog) "/Game/Assets/Dialog/Reventure_PDP_PanneauWood.Reventure_PDP_PanneauWood")
      (Sprite|SetFlipbook (Variables|Default|GetPaperFlipbook) "/Game/Assets/Props/Panneau/FB_Reventure_PanneauWood.FB_Reventure_PanneauWood"))))

(fn BreakPanneau
  (bind _bpc_dialog (Variables|Default|GetBPC_Dialog))
  (bind _bpc_dialog_2 (Variables|Default|GetBPC_Dialog))
  (bind _messagedialog (Variables|/Game/Blueprints/NPC/BPC_Dialog.BPC_Dialog_C|GetMessageDialog _bpc_dialog_2))
  (bind _messagedialog_2 (Variables|/Game/Blueprints/NPC/BPC_Dialog.BPC_Dialog_C|GetMessageDialog _bpc_dialog))
  (bind _returnvalue (Utilities|String|Len _messagedialog_2))
  (if (and (not (Variables|Default|GetisBroken)) (not (Variables|Default|GetisUnbreakable)))
    (Variables|Default|SetisBroken true)
    (Sprite|SetFlipbook (Variables|Default|GetPaperFlipbook) "/Game/Assets/Props/Panneau/FB_Reventure_PanneauWoodBroken.FB_Reventure_PanneauWoodBroken")
    (Default|CloseDialog (Variables|Default|GetBPC_Dialog))
    (LocalVariables|SetDirectionToLaunch (Math|Vector|Normalize (- (Transformation|GetActorLocation (Game|Player|GetPlayerPawn 0)) (Transformation|GetActorLocation))))
    (Utilities|FlowControl|Sequence
      (:then_0
        (bind _returnvalue_2 (Game|SpawnActorfromClass "/Game/Blueprints/NPC/BP_Panneau_Morceaux.BP_Panneau_Morceaux_C" (Math|Transform|MakeTransform (+ (Transformation|GetActorLocation) (* (LocalVariables|GetDirectionToLaunch) 1e+02)) "0, 0, 0" "10.000000,1.000000,10.000000") "Undefined" 0 false 0))
        (bind _output_get (LocalVariables|SetPanneauMorceaux1 _returnvalue_2))
        (Default|SetDialog (Variables|/Game/Blueprints/NPC/BP_Panneau_Morceaux.BP_Panneau_Morceaux_C|GetBPC_Dialog _output_get) (Utilities|String|Append (Utilities|String|GetSubstring _messagedialog 0 (/ (Utilities|String|Len _messagedialog) 2)) " ...")))
      (:then_1
        (bind _returnvalue_3 (Game|SpawnActorfromClass "/Game/Blueprints/NPC/BP_Panneau_Morceaux.BP_Panneau_Morceaux_C" (Math|Transform|MakeTransform (+ (Transformation|GetActorLocation) (* (LocalVariables|GetDirectionToLaunch) 1.5e+02)) "0, 0, 0" "10.000000,1.000000,10.000000") "Undefined" 0 true 0))
        (bind _output_get_2 (LocalVariables|SetPanneauMorceaux2 _returnvalue_3))
        (Default|SetDialog (Variables|/Game/Blueprints/NPC/BP_Panneau_Morceaux.BP_Panneau_Morceaux_C|GetBPC_Dialog _output_get_2) (Utilities|String|Append "... " (Utilities|String|GetSubstring _messagedialog_2 (/ _returnvalue 2) _returnvalue))))
      (:then_2
        (Class|PrimitiveComponent|AddVelocityChangeImpulseatLocation (Variables|/Game/Blueprints/NPC/BP_Panneau_Morceaux.BP_Panneau_Morceaux_C|GetCapsule (LocalVariables|GetPanneauMorceaux1)) (+ (* (LocalVariables|GetDirectionToLaunch) 1.0) (Math|Vector|MakeVector 0.0 0.0 1.0)) "0.000000,0.000000,10.000000" "None")
        (Class|PrimitiveComponent|AddVelocityChangeImpulseatLocation (Variables|/Game/Blueprints/NPC/BP_Panneau_Morceaux.BP_Panneau_Morceaux_C|GetCapsule (LocalVariables|GetPanneauMorceaux2)) (+ (* (LocalVariables|GetDirectionToLaunch) 1.0) (Math|Vector|MakeVector 0.0 0.0 1.0)) "0.000000,0.000000,10.000000" "None")))))