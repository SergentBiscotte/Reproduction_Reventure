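; GM_End is the game mode for the ending screen, showing the last ending stored in GI_GameInfo while epic music plays.
; InitUi creates the W_End widget with the cursor hidden, then BeginPlay runs its level transition and passes it the ending.
; EventCloseTransition reverses the transition, then opens the gallery level when viewing an old or unlocking a new ending, otherwise the game's loading level.
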(event Custom|EventCloseTransition
  (Default|CloseAddEvent (Variables|/Game/UI/W_End.W_End_C|GetW_TransitionLevel (Variables|Default|GetwidgetEndRef)) "Reverse" (delegate Custom|OpenNextLevel)))

(event Custom|OpenNextLevel
  (CallFunction|NextLevel))

(event EventBeginPlay
  (|CallParentFunction)
  (bind _returnvalue (Audio|SpawnSound2D "/Game/Assets/Test/EpicAdventure.EpicAdventure" 1.0 1.0 0.0 0))
  (bind _output_get (Variables|Default|SetactualSoundPlaying _returnvalue))
  (Audio|Components|Audio|Play _output_get 0.0)
  (Default|Close (Variables|/Game/UI/W_End.W_End_C|GetW_TransitionLevel (Variables|Default|GetwidgetEndRef)) "Forward")
  (bind _asgi_game_info (Utilities|Casting|CastToGI_GameInfo (Game|GetGameInstance)))
  (Default|SetEnd (Variables|Default|GetwidgetEndRef) (Variables|/Game/Blueprints/GameInstance/GI_GameInfo.GI_GameInfo_C|GetlastEnd _asgi_game_info)))

(event EventTick
  (params (DeltaSeconds :type Float%20%28single-precision%29))
  (|CallParentFunction DeltaSeconds) ; This node is disabled and will not be called.\nDrag off pins to build functionality.
)

(fn ConstructionScript
  (|CallParentFunction))

(fn InitUi
  (|CallParentFunction)
  (Variables|/Script/Engine.PlayerController|SetbShowMouseCursor (Game|GetPlayerController 0) false)
  (bind _returnvalue (UserInterface|CreateWidget "/Game/UI/W_End.W_End_C"))
  (bind _output_get (Variables|Default|SetwidgetEndRef _returnvalue))
  (UserInterface|Viewport|AddtoViewport _output_get 0))

(fn ReturntoGame
  (bind _asgi_game_info (Utilities|Casting|CastToGI_GameInfo (Game|GetGameInstance)))
  (if (or (Variables|/Game/Blueprints/GameInstance/GI_GameInfo.GI_GameInfo_C|GetisJustLookingOldEnd _asgi_game_info) (Variables|/Game/Blueprints/GameInstance/GI_GameInfo.GI_GameInfo_C|GetisUnlockingNewEnd _asgi_game_info))
    (return "Level_Galerie")
    (else
      (return "Level_LoadingGame"))))

(fn NextLevel
  (bind _nextlevelname (CallFunction|ReturntoGame))
  (Game|OpenLevel(byName) _nextlevelname))