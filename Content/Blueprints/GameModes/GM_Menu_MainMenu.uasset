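; Main menu game mode that creates the menu widget, plays the looping or one-shot menu music and fades in from a white screen on start.
; NextLevel picks the gallery or loading level from the accomplished-ending count in GI_GameInfo, then runs a closing transition widget before opening it.
; Holding Escape shows a quit box while Tick accumulates time, quitting the game after three seconds.
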(event Custom|EventCloseTransition
  (bind _mainmenuref (Variables|Default|GetMainMenuRef))
  (bind _w_transitionlevel (Variables|/Game/UI/W_MainMenu.W_MainMenu_C|GetW_TransitionLevel _mainmenuref))
  (Widget|SetVisibility _w_transitionlevel "Visible")
  (Default|CloseAddEvent _w_transitionlevel "Reverse" (delegate Custom|OpenNextLevel)))

(event Custom|OpenNextLevel
  (Game|OpenLevel(byName) (Variables|Default|GetlevelName)))

(event EventBeginPlay
  (|CallParentFunction)
  (bind _returnvalue (Audio|SpawnSound2D "/Game/Assets/Test/EpicAdventure.EpicAdventure" 1.0 1.0 0.0 0))
  (bind _output_get (Variables|Default|SetactualSoundPlaying _returnvalue))
  (Audio|Components|Audio|Play _output_get 0.0)
  (Default|Fadein (Variables|/Game/UI/W_MainMenu.W_MainMenu_C|GetW_FadeWhiteScreen (Variables|Default|GetMainMenuRef)) "Reverse"))

(event EventTick
  (params (DeltaSeconds :type Float%20%28single-precision%29))
  (|CallParentFunction DeltaSeconds)
  (if (Variables|Default|GetisHoldingEscape)
    (bind _output_get (Variables|Default|SetTimerBeforeQuit (+ (Variables|Default|GetTimerBeforeQuit) (Utilities|Time|GetWorldDeltaSeconds))))
    (if (>= _output_get 3.0)
      (Game|QuitGame 0 "Quit" false))))

(fn ConstructionScript
  (|CallParentFunction))

(fn InitUi
  (|CallParentFunction)
  (bind _returnvalue (UserInterface|CreateWidget "/Game/UI/W_MainMenu.W_MainMenu_C"))
  (bind _output_get (Variables|Default|SetmainMenuRef _returnvalue))
  (UserInterface|Viewport|AddtoViewport _output_get 0))

(fn NextLevel
  (bind _asgi_game_info (Utilities|Casting|CastToGI_GameInfo (Game|GetGameInstance)))
  (if (> (Variables|/Game/Blueprints/GameInstance/GI_GameInfo.GI_GameInfo_C|GetNumberAccomplishedEnd _asgi_game_info) 0)
    (Variables|Default|SetlevelName "Level_Galerie")
    (else
      (Variables|Default|SetlevelName "Level_LoadingGame")))
  (CallFunction|EventCloseTransition))

(fn HoldEscape
  (params (isHolding :type Boolean))
  (bind _output_get (Variables|Default|SetisHoldingEscape isHolding))
  (if _output_get
    (Variables|Default|SetTimerBeforeQuit 0.0)
    (Widget|SetVisibility (Variables|/Game/UI/W_MainMenu.W_MainMenu_C|GetBox_Quit (Variables|Default|GetMainMenuRef)) "Visible")
    (else
      (Widget|SetVisibility (Variables|/Game/UI/W_MainMenu.W_MainMenu_C|GetBox_Quit (Variables|Default|GetMainMenuRef)) "Hidden"))))