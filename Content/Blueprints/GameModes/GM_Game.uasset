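; Game mode for gameplay levels with multiple unlockable endings, handling the day intro, music, pause menu and level exits.
; BeginPlay builds the HUD from GI_GameInfo, then the intro's disappear callback releases the character from cinematic mode and restarts music.
; Pause applies once its widget animation finishes.
; Endings trigger slow motion, get recorded in GI_GameInfo, then leave through a transition widget; play time is saved back on EndPlay.
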(event Custom|PressedButtonWaitingEvent
  (Variables|Default|SetisButtonPressedWaiting true))

(event Custom|StartDayFinishedEvent
  (Variables|Default|SetisStartDayFinished true)
  (bind _asbp_character (Utilities|Casting|CastToBP_Character (Game|Player|GetPlayerPawn 0)))
  (Variables|/Game/Blueprints/BP_Character.BP_Character_C|SetisInCinematicMode _asbp_character false)
  (Default|StartSwitchingZone (Variables|/Game/Blueprints/BP_Character.BP_Character_C|GetPlayerCamera _asbp_character))
  (Audio|Components|Audio|Stop (Variables|Default|GetactualSoundPlaying))
  (bind _returnvalue (Audio|SpawnSound2D "/Game/Assets/Test/EpicAdventure.EpicAdventure" 1.0 1.0 0.0 0))
  (bind _output_get (Variables|Default|SetactualSoundPlaying _returnvalue))
  (Audio|Components|Audio|Play _output_get 0.0))

(event Custom|CloseEventTransition
  (bind _returnvalue (UserInterface|CreateWidget "/Game/UI/Components/W_TransitionLevel.W_TransitionLevel_C"))
  (UserInterface|Viewport|AddtoViewport _returnvalue 10)
  (Default|CloseAddEvent _returnvalue "Reverse" (delegate Custom|OpenNextLevel)))

(event Custom|OpenNextLevel
  (Game|OpenLevel(byName) (Variables|Default|GetnextLevelName)))

(event Custom|PlayPauseAnimation
  (params (gamePaused :type Boolean))
  (bind _wpausemenuref (Variables|Default|GetwPauseMenuRef))
  ;[1 1 1] Animation du menu pause
  (if gamePaused
    (Default|AddEventAppear _wpausemenuref (delegate Custom|PauseAppearFinished))
    (else
      (Default|AddEventDisappear _wpausemenuref (delegate Custom|PauseDisappearFinished)))))

(event Custom|PauseAppearFinished
  ;[1 1 1] Animation du menu pause
  (CallFunction|FinalizedPause true))

(event Custom|PauseDisappearFinished
  ;[1 1 1] Animation du menu pause
  (CallFunction|FinalizedPause false))

(event Custom|TimerUnlockEnd
  (params (NumberEnd :type Integer))
  (Utilities|FlowControl|Delay (* (Class|GameplayStatics|GetGlobalTimeDilation) 1.5))
  (CallFunction|UnlockNewEnd NumberEnd))

(event EventBeginPlay
  (bind _returnvalue (Audio|SpawnSound2D "/Game/Assets/Test/EpicAdventure.EpicAdventure" 1.0 1.0 0.0 0))
  (bind _output_get (Variables|Default|SetactualSoundPlaying _returnvalue))
  (Audio|Components|Audio|Play _output_get 0.0)
  (CallFunction|InitUi)
  (Default|Close (Variables|/Game/UI/W_StartDay.W_StartDay_C|GetW_TransitionLevel (Variables|Default|GetwStartDayRef)) "Forward")
  (Default|BeginTypewriter (Variables|/Game/UI/W_StartDay.W_StartDay_C|GetW_Typewriter (Variables|Default|GetwStartDayRef)))
  (Default|AddPressedButtonWaitingEvent (Variables|Default|GetwStartDayRef) (delegate Custom|PressedButtonWaitingEvent))
  (Default|AddDisappearEvent (Variables|Default|GetwStartDayRef) (delegate Custom|StartDayFinishedEvent)))

(event EventTick
  (params (DeltaSeconds :type Float%20%28single-precision%29))
  (Variables|Default|SetGameTime (+ DeltaSeconds (Variables|Default|GetGameTime))))

(event EventEndPlay
  (params (EndPlayReason :type EEndPlayReason%20Enum :default "Destroyed"))
  (bind _asgi_game_info (Utilities|Casting|CastToGI_GameInfo (Game|GetGameInstance)))
  (Variables|/Game/Blueprints/GameInstance/GI_GameInfo.GI_GameInfo_C|SetGameTime _asgi_game_info (Variables|Default|GetGameTime)))

(fn ConstructionScript)

(fn InitUi
  (Variables|Default|SetisStartDayFinished false)
  (Variables|Default|SetisButtonPressedWaiting false)
  (Utilities|FlowControl|Sequence
    (:then_0
      (bind _returnvalue (UserInterface|CreateWidget "/Game/UI/W_NameZone.W_NameZone_C"))
      (bind _output_get (Variables|Default|SetwNameZoneRef _returnvalue))
      (UserInterface|Viewport|AddtoViewport _output_get 0)
      (bind _asgi_game_info (Utilities|Casting|CastToGI_GameInfo (Game|GetGameInstance)))
      (Default|SetPercentage (Variables|Default|GetwNameZoneRef) (Variables|/Game/Blueprints/GameInstance/GI_GameInfo.GI_GameInfo_C|GetNumberAccomplishedEnd _asgi_game_info)))
    (:then_1
      (bind _returnvalue_2 (UserInterface|CreateWidget "/Game/UI/W_StartDay.W_StartDay_C"))
      (bind _output_get_2 (Variables|Default|SetwStartDayRef _returnvalue_2))
      (UserInterface|Viewport|AddtoViewport _output_get_2 1)
      (bind _asgi_game_info_2 (Utilities|Casting|CastToGI_GameInfo (Game|GetGameInstance)))
      (Default|SetDayYear (Variables|Default|GetwStartDayRef) (Variables|/Game/Blueprints/GameInstance/GI_GameInfo.GI_GameInfo_C|GetactualYear _asgi_game_info_2) (Variables|/Game/Blueprints/GameInstance/GI_GameInfo.GI_GameInfo_C|GetactualDay _asgi_game_info_2))
      (if (>= (.number (Variables|/Game/Blueprints/GameInstance/GI_GameInfo.GI_GameInfo_C|GetlastEnd _asgi_game_info_2)) 1)
        (bind _newtext (Default|ReplacePlayerName _asgi_game_info_2 (.newdaytext (Variables|/Game/Blueprints/GameInstance/GI_GameInfo.GI_GameInfo_C|GetlastEnd _asgi_game_info_2))))
        (Default|SetTexttoWrite (Variables|Default|GetwStartDayRef) _newtext)
        (else
          (bind _newtext_2 (Default|ReplacePlayerName _asgi_game_info_2 "Tout commença par un jour plutôt normal de la vie de {0}..."))
          (Default|SetTexttoWrite (Variables|Default|GetwStartDayRef) _newtext_2))))
    (:then_2
      (bind _returnvalue_3 (UserInterface|CreateWidget "/Game/UI/W_PauseMenu.W_PauseMenu_C"))
      (bind _output_get_3 (Variables|Default|SetwPauseMenuRef _returnvalue_3))
      (UserInterface|Viewport|AddtoViewport _output_get_3 2)
      (CallFunction|SetPause false)
      (Widget|SetVisibility (Variables|Default|GetwPauseMenuRef) "Hidden")
      (bind _asgi_game_info_3 (Utilities|Casting|CastToGI_GameInfo (Game|GetGameInstance)))
      (Variables|Default|SetGameTime (Variables|/Game/Blueprints/GameInstance/GI_GameInfo.GI_GameInfo_C|GetGameTime _asgi_game_info_3)))))

(fn SetPause
  (params (isGamePaused :type Boolean))
  (if isGamePaused
    (Widget|SetVisibility (Variables|Default|GetwPauseMenuRef) "Visible"))
  (CallFunction|PlayPauseAnimation isGamePaused))

(fn PressedButton
  (Default|PlayDisappear (Variables|Default|GetwStartDayRef) "Forward"))

(fn NavigationWidget
  (params (direction :type E_WidgetNavigationDirection%20Enum :default "NewEnumerator0"))
  (if (Variables|Default|GetisGamePaused)
    (Class|BPIWidgetGamepadNavigation|GetNavigationInput(Message) (Variables|Default|GetwPauseMenuRef) direction)))

(fn ReturntoMenu
  (Utilities|FlowControl|Sequence
    (:then_0
      (bind _asgi_game_info (Utilities|Casting|CastToGI_GameInfo (Game|GetGameInstance)))
      (if (>= (Variables|/Game/Blueprints/GameInstance/GI_GameInfo.GI_GameInfo_C|GetNumberAccomplishedEnd _asgi_game_info) 1)
        (Variables|Default|SetnextLevelName "Level_Galerie")
        (else
          (Variables|Default|SetnextLevelName "Level_MainMenu"))))
    (:then_1
      (CallFunction|CloseEventTransition))))

(fn FinalizedPause
  (params (gamePaused :type Boolean))
  (Variables|Default|SetisGamePaused gamePaused)
  (if (Variables|Default|GetisGamePaused)
    (Widget|SetVisibility (Variables|Default|GetwPauseMenuRef) "Visible")
    (Variables|/Script/Engine.PlayerController|SetbShowMouseCursor (Game|GetPlayerController 0) true)
    (Game|SetGamePaused true)
    (Default|SetTimeinGame (Variables|Default|GetwPauseMenuRef) (Variables|Default|GetGameTime))
    (bind _asgi_game_info (Utilities|Casting|CastToGI_GameInfo (Game|GetGameInstance)))
    (Default|SetNumberEnds (Variables|Default|GetwPauseMenuRef) (Variables|/Game/Blueprints/GameInstance/GI_GameInfo.GI_GameInfo_C|GetNumberAccomplishedEnd _asgi_game_info))
    (else
      (Widget|SetVisibility (Variables|Default|GetwPauseMenuRef) "Hidden")
      (Variables|/Script/Engine.PlayerController|SetbShowMouseCursor (Game|GetPlayerController 0) false)
      (Game|SetGamePaused false))))

(fn UnlockNewEnd
  (params (endNumber :type Integer))
  (CallFunction|SetGlobalTimeDilation 1.0)
  (bind _asgi_game_info (Utilities|Casting|CastToGI_GameInfo (Game|GetGameInstance)))
  (Default|UnlockNewEnd _asgi_game_info endNumber)
  (Variables|Default|SetnextLevelName "LVL_End_1")
  (CallFunction|CloseEventTransition))

(fn SetGlobalTimeDilation
  (params (timeDilation :type Float%20%28double-precision%29))
  (Utilities|Time|SetGlobalTimeDilation timeDilation))

(fn UnlockNewEndTimer
  (params (EndNumber :type Integer))
  (CallFunction|SetGlobalTimeDilation 0.2)
  (CallFunction|TimerUnlockEnd EndNumber))