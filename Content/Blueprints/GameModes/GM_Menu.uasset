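; Base game mode for menu levels that sets up mouse input and defines hooks for child GM_Menu_ variants.
; On BeginPlay, InitUi calls EnableMouse, which switches the player controller between Game-and-UI input with a visible cursor and Game-Only input without one.
; NextLevel only prints an error unless overridden, and NavigationWidget is an empty stub taking a direction.
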(event EventBeginPlay
  (CallFunction|InitUi))

(event EventTick
  (params (DeltaSeconds :type Float%20%28single-precision%29)))

(fn ConstructionScript)

(fn InitUi
  (CallFunction|EnableMouse true))

(fn EnableMouse
  (params (isMouseEnabled :type Boolean))
  (if isMouseEnabled
    ;[1 1 1] Enable Mouse
    (Input|SetInputModeGameandUI (Game|GetPlayerController 0) 0 "DoNotLock" false false)
    (Variables|/Script/Engine.PlayerController|SetbShowMouseCursor (Game|GetPlayerController 0) true)
    (else
      ;[1 1 1] Disable Mouse
      (Input|SetInputModeGameOnly (Game|GetPlayerController 0) false)
      (Variables|/Script/Engine.PlayerController|SetbShowMouseCursor (Game|GetPlayerController 0) false))))

(fn NextLevel
  (Development|PrintString "Error: NextLevel isn't override by GM_Menu_..."))

(fn NavigationWidget
  (params (direction :type E_WidgetNavigationDirection%20Enum :default "NewEnumerator0")))