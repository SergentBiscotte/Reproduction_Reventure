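; Game mode for the splash screen level, which shows the splash widget and then loads the main menu.
; InitUi creates W_SplashingScreen and adds it to the viewport.
; BeginPlay plays the widget's white-screen fade in reverse, waits briefly, then plays it forward.
; Each fade ends in a callback event, and the last one opens Level_MainMenu.
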(event Custom|OpenSplashScreenFinished
  (Utilities|FlowControl|Delay 1.5)
  (Default|FadeinAddEvent (Variables|/Game/UI/W_SplashingScreen.W_SplashingScreen_C|GetW_FadeWhiteScreen (Variables|Default|GetSplashScreenRef)) "Forward" (delegate Custom|CloseSplashScreenFinished)))

(event Custom|CloseSplashScreenFinished
  (CallFunction|NextLevel))

(event EventBeginPlay
  (|CallParentFunction)
  (Default|FadeinAddEvent (Variables|/Game/UI/W_SplashingScreen.W_SplashingScreen_C|GetW_FadeWhiteScreen (Variables|Default|GetSplashScreenRef)) "Reverse" (delegate Custom|OpenSplashScreenFinished)))

(event EventTick
  (params (DeltaSeconds :type Float%20%28single-precision%29))
  (|CallParentFunction DeltaSeconds) ; This node is disabled and will not be called.\nDrag off pins to build functionality.
)

(fn ConstructionScript
  (|CallParentFunction))

(fn InitUi
  (|CallParentFunction)
  (bind _returnvalue (UserInterface|CreateWidget "/Game/UI/W_SplashingScreen.W_SplashingScreen_C"))
  (bind _output_get (Variables|Default|SetSplashScreenRef _returnvalue))
  (UserInterface|Viewport|AddtoViewport _output_get 0))

(fn NextLevel
  (Game|OpenLevel(byName) "Level_MainMenu"))