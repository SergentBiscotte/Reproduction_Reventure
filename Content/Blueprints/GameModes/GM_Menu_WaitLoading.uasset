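; Game mode for an intermediate loading level that displays a loading screen, then opens Level_Game.
; InitUi creates the W_LoadingScreen widget, and BeginPlay sets its French title from the last ending stored in GI_GameInfo, clearing its unlock flags.
; The widget's vanish animation plays in reverse to appear, holds briefly, then plays forward, with completion callbacks chaining through to the level change.
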(event Custom|AppearLoadingScreenFinished
  (Utilities|FlowControl|Delay 2.0)
  (Default|VanishLoadingScreenAddEvent (Variables|Default|GetloadingScreenRef) "Forward" (delegate Custom|VanishLoadingScreenFinish)))

(event Custom|VanishLoadingScreenFinish
  (CallFunction|NextLevel))

(event EventBeginPlay
  (|CallParentFunction)
  (Default|VanishLoadingScreenAddEvent (Variables|Default|GetloadingScreenRef) "Reverse" (delegate Custom|AppearLoadingScreenFinished))
  (bind _asgi_game_info (Utilities|Casting|CastToGI_GameInfo (Game|GetGameInstance)))
  (if (!= (.number (Variables|/Game/Blueprints/GameInstance/GI_GameInfo.GI_GameInfo_C|GetlastEnd _asgi_game_info)) 0)
    (Variables|/Game/Blueprints/GameInstance/GI_GameInfo.GI_GameInfo_C|SetisUnlockingNewEnd _asgi_game_info false)
    (if (Variables|/Game/Blueprints/GameInstance/GI_GameInfo.GI_GameInfo_C|GetisAlreadyUnlockEnd _asgi_game_info)
      (Variables|/Game/Blueprints/GameInstance/GI_GameInfo.GI_GameInfo_C|SetisAlreadyUnlockEnd _asgi_game_info false)
      (Default|SetTitleandSubTitle (Variables|Default|GetloadingScreenRef) "Après ce rapide souvenir..." "Chargement")
      (else
        (Default|SetTitleandSubTitle (Variables|Default|GetloadingScreenRef) (.newdayloadingtext (Variables|/Game/Blueprints/GameInstance/GI_GameInfo.GI_GameInfo_C|GetlastEnd _asgi_game_info)) "Chargement")))
    (else
      (Default|SetTitleandSubTitle (Variables|Default|GetloadingScreenRef) "" "Chargement"))))

(event EventTick
  (params (DeltaSeconds :type Float%20%28single-precision%29))
  (|CallParentFunction DeltaSeconds) ; This node is disabled and will not be called.\nDrag off pins to build functionality.
)

(fn ConstructionScript
  (|CallParentFunction))

(fn InitUi
  (|CallParentFunction)
  (bind _returnvalue (UserInterface|CreateWidget "/Game/UI/W_LoadingScreen.W_LoadingScreen_C"))
  (bind _output_get (Variables|Default|SetloadingScreenRef _returnvalue))
  (UserInterface|Viewport|AddtoViewport _output_get 0))

(fn NextLevel
  (Game|OpenLevel(byName) "Level_Game"))