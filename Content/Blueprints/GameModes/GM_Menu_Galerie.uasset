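; Game mode for the gallery menu, where players browse the game's endings, see titles and clues, and replay unlocked ones.
; It creates the W_Galerie widget, forwards navigation input to it, and fills it from ending data in GI_GameInfo, substituting the player name.
; On BeginPlay it starts music, plays the transition and triggers any pending unlock.
; Level changes store a target name, then open it through the transition widget's close event.
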(event Custom|CloseEventTransition
  (Default|CloseAddEvent (Variables|/Game/UI/W_Galerie.W_Galerie_C|GetW_TransitionLevel (Variables|Default|GetmenuGalerieRef)) "Reverse" (delegate Custom|OpenLevel)))

(event Custom|OpenLevel
  (Game|OpenLevel(byName) (Variables|Default|GetlevelName)))

(event Custom|OpenLevel_Game
  (CallFunction|SetLevelName "Level_LoadingGame")
  (CallFunction|NextLevel))

(event Custom|OpenLevel_Menu
  (CallFunction|SetLevelName "Level_MainMenu")
  (CallFunction|NextLevel))

(event EventBeginPlay
  (|CallParentFunction)
  (bind _returnvalue (Audio|SpawnSound2D "/Game/Assets/Test/EpicAdventure.EpicAdventure" 1.0 1.0 0.0 0))
  (bind _output_get (Variables|Default|SetactualSoundPlaying _returnvalue))
  (Audio|Components|Audio|Play _output_get 0.0)
  (Default|Close (Variables|/Game/UI/W_Galerie.W_Galerie_C|GetW_TransitionLevel (Variables|Default|GetmenuGalerieRef)) "Forward")
  (bind _asgi_game_info (Utilities|Casting|CastToGI_GameInfo (Game|GetGameInstance)))
  (Variables|/Game/Blueprints/GameInstance/GI_GameInfo.GI_GameInfo_C|SetisJustLookingOldEnd _asgi_game_info false)
  (if (Variables|/Game/Blueprints/GameInstance/GI_GameInfo.GI_GameInfo_C|GetisUnlockingNewEnd _asgi_game_info)
    (Default|UnlockNewEnd (Variables|Default|GetmenuGalerieRef) (.number (Variables|/Game/Blueprints/GameInstance/GI_GameInfo.GI_GameInfo_C|GetlastEnd _asgi_game_info)))))

(event EventTick
  (params (DeltaSeconds :type Float%20%28single-precision%29))
  (|CallParentFunction DeltaSeconds) ; This node is disabled and will not be called.\nDrag off pins to build functionality.
)

(fn ConstructionScript
  (|CallParentFunction))

(fn InitUi
  (|CallParentFunction)
  (bind _returnvalue (UserInterface|CreateWidget "/Game/UI/W_Galerie.W_Galerie_C" (Game|GetPlayerController 0)))
  (bind _output_get (Variables|Default|SetmenuGalerieRef _returnvalue))
  (UserInterface|Viewport|AddtoViewport _output_get 0)
  (bind _asgi_game_info (Utilities|Casting|CastToGI_GameInfo (Game|GetGameInstance)))
  (Default|SetNumberEndAccomplished (Variables|Default|GetmenuGalerieRef) (Variables|/Game/Blueprints/GameInstance/GI_GameInfo.GI_GameInfo_C|GetNumberAccomplishedEnd _asgi_game_info)))

(fn NextLevel
  (CallFunction|CloseEventTransition))

(fn SetLevelName
  (params (name :type Name))
  (Variables|Default|SetlevelName name))

(fn NavigationWidget
  (params (direction :type E_WidgetNavigationDirection%20Enum :default "NewEnumerator0"))
  (Class|BPIWidgetGamepadNavigation|GetNavigationInput(Message) (Variables|Default|GetmenuGalerieRef) direction))

(fn SetInfoEndWidget
  (params (index :type Integer))
  (bind _asgi_game_info (Utilities|Casting|CastToGI_GameInfo (Game|GetGameInstance)))
  (bind _end (CallFunction|GetEndbyNumber index (Variables|/Game/Blueprints/GameInstance/GI_GameInfo.GI_GameInfo_C|GetEndTab _asgi_game_info)))
  (bind _output_get (LocalVariables|SetactualEnd _end))
  (bind _newtext (Default|ReplacePlayerName _asgi_game_info (.titre _output_get)))
  (Default|SetTitle (Variables|Default|GetmenuGalerieRef) _newtext (.number _output_get) (.isunlock _output_get))
  (bind _newtext_2 (Default|ReplacePlayerName _asgi_game_info (.clue _output_get)))
  (Default|SetClue (Variables|Default|GetmenuGalerieRef) _newtext_2 (.isunlock _output_get)))

(fn LaunchEnd
  (params (end :type STR%20End%20Structure))
  (if (.isunlock end)
    (CallFunction|SetLevelName (.mapendname end))
    (CallFunction|NextLevel)))