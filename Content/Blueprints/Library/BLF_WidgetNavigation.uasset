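; Blueprint function library for gamepad and keyboard navigation between UI widgets.
; TranslateKeyToWidgetNavigation maps stick and arrow keys to a direction enum, with a fallback value for other keys.
; GetNextWidget uses that direction and the current widget's display name to look up its neighbor in nested maps.
; ChangeStyleButton and ChangeStyleButtonRevert are identical toggles, swapping a button's Normal and Hovered brushes to show or clear a highlight.
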(fn TranslateKeytoWidgetNavigation
  (params (Key :type Key%20Structure :default "None"))
  (if (Math|Boolean|ORBoolean (== Key "Gamepad_LeftStick_Left") (== Key "Gamepad_RightStick_Left") (== Key "Left"))
    (return "NewEnumerator1")
    (elif (Math|Boolean|ORBoolean (== Key "Gamepad_LeftStick_Right") (== Key "Gamepad_RightStick_Right") (== Key "Right"))
      (return "NewEnumerator3")
      (elif (Math|Boolean|ORBoolean (== Key "Gamepad_LeftStick_Up") (== Key "Gamepad_RightStick_Up") (== Key "Up"))
        (return "NewEnumerator0")
        (elif (Math|Boolean|ORBoolean (== Key "Gamepad_LeftStick_Down") (== Key "Gamepad_RightStick_Down") (== Key "Down"))
          (return "NewEnumerator2")
          (else
            (return "NewEnumerator4")))))))

(fn GetNextWidget
  (params (direction :type E_WidgetNavigationDirection%20Enum :default "NewEnumerator0") (listWidget :type Map%20of%20Strings%20to%20Structs) (currentWidget :type Widget%20Object%20Reference))
  (bind _returnvalue (Utilities|GetDisplayName currentWidget))
  (bind (_value _returnvalue_2) (Utilities|Map|Find listWidget _returnvalue))
  (bind _navigationlist (Utilities|Struct|BreakSTR_WidgetNavigation _value))
  (bind (_value_2 _returnvalue_3) (Utilities|Map|Find _navigationlist direction))
  (LocalVariables|SetnextWidgetFound 0)
  (Utilities|FlowControl|Sequence
    (:then_0
      (if _returnvalue_2
        (if _returnvalue_3
          (LocalVariables|SetnextWidgetFound _value_2))))
    (:then_1
      (return (LocalVariables|GetnextWidgetFound)))))

(fn ChangeStyleButton
  (params (button :type Button%20Object%20Reference))
  (bind _widgetstyle (Variables|/Script/UMG.Button|GetWidgetStyle button))
  (Utilities|IsValid button
    (:Is%20Valid
      (Class|Button|SetStyle button (Utilities|Struct|MakeButtonStyle (.hovered _widgetstyle) (.normal _widgetstyle) (.pressed _widgetstyle) (.disabled _widgetstyle) (.normalforeground _widgetstyle) (.hoveredforeground _widgetstyle) (.pressedforeground _widgetstyle) (.disabledforeground _widgetstyle) (.normalpadding _widgetstyle) (.pressedpadding _widgetstyle) (.pressedslatesound _widgetstyle) (.hoveredslatesound _widgetstyle))))))

(fn ChangeStyleButtonRevert
  (params (button :type Button%20Object%20Reference))
  (bind _widgetstyle (Variables|/Script/UMG.Button|GetWidgetStyle button))
  (Utilities|IsValid button
    (:Is%20Valid
      (Class|Button|SetStyle button (Utilities|Struct|MakeButtonStyle (.hovered _widgetstyle) (.normal _widgetstyle) (.pressed _widgetstyle) (.disabled _widgetstyle) (.normalforeground _widgetstyle) (.hoveredforeground _widgetstyle) (.pressedforeground _widgetstyle) (.disabledforeground _widgetstyle) (.normalpadding _widgetstyle) (.pressedpadding _widgetstyle) (.pressedslatesound _widgetstyle) (.hoveredslatesound _widgetstyle))))))