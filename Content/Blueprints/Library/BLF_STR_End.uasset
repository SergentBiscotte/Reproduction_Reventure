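; BLF_STR_End is a Blueprint function library for looking up and updating game ending records (title, description, clue, map, media, unlock state) in an array.
; GetEndByNumber loops through the array and returns the first entry whose Number matches the given index, or an empty result otherwise.
; SetEndByNumber overwrites any entry sharing the supplied ending's Number with that ending's fields, and adds nothing when none matches.
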(fn GetEndbyNumber
  (params (index :type Integer) (endTab :type Array%20of%20STR%20End%20Structures))
  (for _array_element endTab
    (if (== (.Number (Utilities|Struct|BreakSTR_End _array_element)) index)
      (return _array_element)))
  (return ""))

(fn SetEndbyNumber
  (params (endTab :type Array%20of%20STR%20End%20Structures) (endToSet :type STR%20End%20Structure))
  (bind (_array_element _array_index) (Utilities|Array|ForEachLoopwithBreak endTab)
    (:LoopBody
      (if (== (.number _array_element) (.number endToSet))
        (Utilities|Array|SetArrayElem endTab _array_index (Utilities|Struct|MakeSTR_End (.number endToSet) (.titre endToSet) (.description endToSet) (.clue endToSet) (.mapendname endToSet) (.endpicture endToSet) (.year endToSet) (.day endToSet) (.newdaytext endToSet) (.newdayloadingtext endToSet) (.isunlock endToSet) (.mediaplayer endToSet) (.videosource endToSet) (.videomaterial endToSet)))))))